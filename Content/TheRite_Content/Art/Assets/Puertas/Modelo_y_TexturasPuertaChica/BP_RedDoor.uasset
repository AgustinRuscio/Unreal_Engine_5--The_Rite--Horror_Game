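; BP_RedDoor is an interactable red door that opens once and sends the player to another level.
; Interaction disables player input, plays sounds and runs timelines that turn both latch handles and swing the door 90 degrees.
; When the swing ends, an open sound plays and a second timeline delays a FadeOut level sequence, whose finish event opens the target level.
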(event Custom|CustomEvent
  (Game|OpenLevel(byObjectReference) (Variables|Default|GetLevel)))

(event Custom|Latch%20Anim
  ;[1 1 1] Anim latch
  (bind _a (Timeline|Timeline PlayFromStart)
    (:Update
      (Transformation|SetRelativeRotation (Variables|Default|GetFront%20Handle) (Math|Rotator|MakeRotator 0.0 (Math|Float|Lerp 5.0 5e+01 _a) 0.0) false false)
      (Transformation|SetRelativeRotation (Variables|Default|GetBack%20Handle) (Math|Rotator|MakeRotator -1.8e+02 (Math|Float|Lerp 5.0 5e+01 _a) 0.0) false false))))

(event EventInteraction
  (if (not (Variables|Default|GetAlReadyOpen))
    (Variables|Default|SetAlReadyOpen true)
    (Input|DisableInput (Game|Player|GetPlayerPawn 0) 0)
    (CallFunction|LatchAnim)
    (Audio|SpawnSound2D 0 1.0 1.0 0.0 0)
    (Audio|PlaySoundatLocation "/Game/TheRite_Content/Sound/SoundFX/SFX_DoorLocked.SFX_DoorLocked" "0, 0, 0" "0, 0, 0" 1.0 1.0 0.0 0 0 0 0)
    (bind _doorfloat (Timeline|AnimationTimeLine Play)
      (:Update
        (Transformation|SetRelativeRotation (Variables|Default|GetDoor) (Math|Rotator|MakeRotator 0.0 0.0 (Math|Float|Lerp 0.0 9e+01 _doorfloat)) false false))
      (:Finished
        (Audio|SpawnSound2D "/Game/TheRite_Content/Sound/SoundFX/SFX_RedDoorOpen.SFX_RedDoorOpen" 1.0 1.0 0.0 0)
        (Timeline|ChangeLevel%20Time%20Line Play
          (:Finished
            (bind _outactor (Sequencer|Player|CreateLevelSequencePlayer "/Game/TheRite_Content/Sequencecs/FadeOut.FadeOut"))
            (Sequencer|Player|Play (Variables|/Script/LevelSequence.LevelSequenceActor|GetSequencePlayer _outactor) :!class /Script/MovieScene.MovieSceneSequencePlayer)
            (EventDispatchers|BindEventtoOnFinished (Variables|/Script/LevelSequence.LevelSequenceActor|GetSequencePlayer _outactor) (delegate Custom|CustomEvent))))))))

(fn ConstructionScript)