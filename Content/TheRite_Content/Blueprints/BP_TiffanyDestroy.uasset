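; BP_TiffanyDestroy is a one-shot trigger box that fires when BP_Alex overlaps it.
; A sequence unlocks every entry in an array, starts a delayed BP_Tiffany lookup whose result goes unused, and plays a timeline scaling a rect light's current intensity.
; The final branch destroys the trigger immediately, without waiting for the delay or timeline to finish.
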(event OnComponentBeginOverlap(Box)
  (params (OverlappedComponent :type Primitive%20Component%20Object%20Reference) (OtherActor :type Actor%20Object%20Reference) (OtherComp :type Primitive%20Component%20Object%20Reference) (OtherBodyIndex :type Integer) (bFromSweep :type Boolean) (SweepResult :type Hit%20Result%20Structure%20%28by%20ref%29))
  (bind _light (Variables|Default|GetLight))
  (bind _rectlight (Variables|/Game/TheRite_Content/Blueprints/BP_Light.BP_Light_C|GetRectLight _light))
  (Utilities|Casting|CastToBP_Alex OtherActor)
  (Utilities|FlowControl|Sequence
    (:then_0
      (for _array_element (Variables|Default|GetNewVar)
        (Variables|/Game/TheRite_Content/Blueprints/BP_Door.BP_Door_C|SetIsLocked _array_element false)))
    (:then_1
      (Utilities|FlowControl|Delay 0.7)
      (Actor|GetActorOfClass "/Game/TheRite_Content/Blueprints/Character/BP_Tiffany.BP_Tiffany_C"))
    (:then_2
      (bind _newtrack_0 (Timeline|Timeline Play)
        (:Update
          (Rendering|Components|Light|SetIntensity _rectlight (* _newtrack_0 (Variables|/Script/Engine.LightComponentBase|GetIntensity _rectlight))))))
    (:then_3
      (Actor|DestroyActor))))

(fn ConstructionScript)