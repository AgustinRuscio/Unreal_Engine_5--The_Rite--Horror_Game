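; Interactive drawer that alternates between sliding open and closed on each interaction, firing OnDrawerOpen when it opens.
; Open and Close timelines move the root along MoveDir, lerping from its current location each update rather than a stored start.
; CanInteract blocks input until each timeline finishes.
; A separate AddingForce event enables mesh physics, launches it along ForceDir, then destroys the actor after a Wait timeline.
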(event Custom|AddingForce
  (bind _staticmesh (Variables|Default|GetStaticMesh))
  ;[1 1 1] AddinG Force
  (Physics|SetSimulatePhysics _staticmesh true)
  (Physics|AddForce _staticmesh (* (Variables|Default|GetForceDir) (Variables|Default|GetForceIntensity)) "None" true)
  (Timeline|wait PlayFromStart
    (:Finished
      (Actor|DestroyActor self))))

(event EventInteraction
  (bind _defaultsceneroot (Variables|Default|GetDefaultSceneRoot))
  (bind _defaultsceneroot_2 (Variables|Default|GetDefaultSceneRoot))
  (bind _defaultsceneroot_3 (Variables|Default|GetDefaultSceneRoot))
  (bind _relativelocation (Variables|/Script/Engine.SceneComponent|GetRelativeLocation _defaultsceneroot_3))
  (bind _relativelocation_2 (Variables|/Script/Engine.SceneComponent|GetRelativeLocation _defaultsceneroot_2))
  (if (Variables|Default|GetCanInteract)
    (Utilities|FlowControl|FlipFlop
      (:A
        (Default|CallOnDrawerOpen self)
        (Variables|Default|SetCanInteract false)
        (bind _newtrack_0 (Timeline|Open PlayFromStart)
          (:Update
            (Transformation|SetRelativeLocation _defaultsceneroot (Math|Vector|Lerp(Vector) _relativelocation (+ _relativelocation (Variables|Default|GetMoveDir)) _newtrack_0) false false)
            (Development|PrintString "opening"))
          (:Finished
            (Variables|Default|SetCanInteract true :!label _label)
            (Development|PrintString "finished"))))
      (:B
        (Variables|Default|SetCanInteract false)
        (bind _newtrack_0_2 (Timeline|Close PlayFromStart)
          (:Update
            (Transformation|SetRelativeLocation _defaultsceneroot (Math|Vector|Lerp(Vector) _relativelocation_2 (- _relativelocation_2 (Variables|Default|GetMoveDir)) _newtrack_0_2) false false)
            (Development|PrintString "closing"))
          (:Finished
            (goto _label)))))))

(fn ConstructionScript)