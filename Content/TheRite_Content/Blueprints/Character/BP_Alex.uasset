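; BP_Alex is the player character, handling Enhanced Input movement, sprint, pause menu, hint display and interaction.
; Tick drives a timed lighter with cooldown, speed-based head-bob shakes, periodic breathing audio and an all-items-collected dispatch.
; A per-frame camera sphere trace finds IInteractuable actors, setting the interaction target and center-dot UI, with special cases for locked doors and portraits.
; Lighter state changes fire a dispatcher that toggles its montage and meshes.
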(event Custom|Montage%20Animation%20On%20Off
  (bind _lighter (Variables|Default|GetLighter))
  (if (Variables|Flashlight|GetFlashlight)
    (Animation|PlayAnimMontage "/Game/TheRite_Content/Art/Models/Alex/NewModel/A_Lighter_Montage.A_Lighter_Montage" 1.0 "None")
    (Rendering|SetVisibility _lighter true false)
    (else
      (Animation|StopAnimMontage "/Game/TheRite_Content/Art/Models/Alex/NewModel/A_Lighter_Montage.A_Lighter_Montage")
      (Rendering|SetVisibility _lighter false false))))

(event Custom|HeadBob
  (bind _returnvalue (Game|GetPlayerController 0))
  (bind _returnvalue_2 (Transformation|GetVelocity))
  (bind _returnvalue_3 (Math|Vector|VectorLength _returnvalue_2))
  ;[1 1 1] HeadBob
  (if (> _returnvalue_3 0.0)
    (if (< _returnvalue_3 7e+02)
      (Game|Feedback|ClientStartCameraShake _returnvalue "/Game/TheRite_Content/Blueprints/Others/CameraShake_Walk.CameraShake_Walk_C" 1.0 "CameraLocal" "0, 0, 0")
      (else
        (Game|Feedback|ClientStartCameraShake _returnvalue "/Game/TheRite_Content/Blueprints/Others/CameraShake_Run.CameraShake_Run_C" 1.0 "CameraLocal" "0, 0, 0")))
    (else
      (Game|Feedback|ClientStartCameraShake _returnvalue "/Game/TheRite_Content/Blueprints/Others/CameraShake_Idle.CameraShake_Idle_C" 1.0 "CameraLocal" "0, 0, 0"))))

(event Input|EnhancedActionEvents|EnhancedInputActionAlex_Look
  (params (ActionValue :type Vector%202D%20Structure) (ElapsedSeconds :type Float%20%28double-precision%29) (TriggeredSeconds :type Float%20%28double-precision%29) (InputAction :type Input%20Action%20Object%20Reference :default "/Game/TheRite_Content/Input/Input_Actions/Alex_Look.Alex_Look"))
  ;[1 1 1] Inputs
  ;;[1 1 1] Move Camera
  (:Triggered
    (Pawn|Input|AddControllerYawInput (.x ActionValue))
    (Pawn|Input|AddControllerPitchInput (.y ActionValue))))

(event Input|EnhancedActionEvents|EnhancedInputActionAlex_Move
  (params (ActionValue :type Vector%202D%20Structure) (ElapsedSeconds :type Float%20%28double-precision%29) (TriggeredSeconds :type Float%20%28double-precision%29) (InputAction :type Input%20Action%20Object%20Reference :default "/Game/TheRite_Content/Input/Input_Actions/Alex_Move.Alex_Move"))
  ;[1 1 1] Inputs
  ;;[1 1 1] Move Character
  (:Triggered
    (Pawn|Input|AddMovementInput (Transformation|GetActorRightVector) (.x ActionValue) false)
    (Pawn|Input|AddMovementInput (Transformation|GetActorForwardVector) (.y ActionValue) false)))

(event Input|EnhancedActionEvents|EnhancedInputActionAlex_Spint
  (params (ActionValue :type Boolean) (ElapsedSeconds :type Float%20%28double-precision%29) (TriggeredSeconds :type Float%20%28double-precision%29) (InputAction :type Input%20Action%20Object%20Reference :default "/Game/TheRite_Content/Input/Input_Actions/Alex_Spint.Alex_Spint"))
  ;[1 1 1] Inputs
  ;;[1 1 1] Sprint
  (:Triggered
    (CallFunction|StartSprint))
  (:Completed
    (CallFunction|StopSprint)))

(event Input|EnhancedActionEvents|EnhancedInputActionAlex_Interaction
  (params (ActionValue :type Boolean) (ElapsedSeconds :type Float%20%28double-precision%29) (TriggeredSeconds :type Float%20%28double-precision%29) (InputAction :type Input%20Action%20Object%20Reference :default "/Game/TheRite_Content/Input/Input_Actions/Alex_Interaction.Alex_Interaction"))
  ;[1 1 1] Inputs
  ;;[1 1 1] Use interactuable
  (:Started
    (if (Variables|Interactions|GetCanInteract)
      (Default|Interaction (Variables|Interactions|GetActualnteractuable)))))

(event Input|EnhancedActionEvents|EnhancedInputActionAlex_Flashlight
  (params (ActionValue :type Boolean) (ElapsedSeconds :type Float%20%28double-precision%29) (TriggeredSeconds :type Float%20%28double-precision%29) (InputAction :type Input%20Action%20Object%20Reference :default "/Game/TheRite_Content/Input/Input_Actions/Alex_Flashlight.Alex_Flashlight"))
  ;[1 1 1] Inputs
  ;;[1 1 1] Turn on Lighter (if possible)
  (:Started
    (if (Variables|Default|GetCanUseFlashLight)
      (CallFunction|CheckLighterON))))

(event Input|EnhancedActionEvents|EnhancedInputActionAlex_OpenHint
  (params (ActionValue :type Boolean) (ElapsedSeconds :type Float%20%28double-precision%29) (TriggeredSeconds :type Float%20%28double-precision%29) (InputAction :type Input%20Action%20Object%20Reference :default "/Game/TheRite_Content/Input/Input_Actions/Alex_OpenHint.Alex_OpenHint"))
  (bind _hint (Variables|Default|GetHint))
  (bind _hashint (Variables|Default|GetHasHint))
  ;[1 1 1] Inputs
  ;;[1 1 1] Open Hints
  (:Triggered
    (if _hashint
      (Animation|PlayAnimMontage "/Game/TheRite_Content/Art/Models/Alex/NewModel/A_Hint_Alex_Montage.A_Hint_Alex_Montage" 1.0 "None")
      (Rendering|SetVisibility _hint true false)))
  (:Canceled
    (if _hashint :!label _label
      (Animation|StopAnimMontage "/Game/TheRite_Content/Art/Models/Alex/NewModel/A_Hint_Alex_Montage.A_Hint_Alex_Montage")
      (Rendering|SetVisibility _hint false false)))
  (:Completed
    (goto _label)))

(event Input|EnhancedActionEvents|EnhancedInputActionAlex_Pause
  (params (ActionValue :type Boolean) (ElapsedSeconds :type Float%20%28double-precision%29) (TriggeredSeconds :type Float%20%28double-precision%29) (InputAction :type Input%20Action%20Object%20Reference :default "/Game/TheRite_Content/Input/Input_Actions/Alex_Pause.Alex_Pause"))
  (bind _puasemenu (Variables|Default|GetPuaseMenu))
  ;[1 1 1] Inputs
  ;;[1 1 1] Puase game
  (:Started
    (Utilities|FlowControl|FlipFlop
      (:A
        (Widget|SetVisibility _puasemenu "Visible")
        (Game|SetGamePaused true))
      (:B
        (Widget|SetVisibility _puasemenu "Hidden")
        (Game|SetGamePaused false)))))

(event EventBeginPlay
  (Utilities|FlowControl|Sequence
    (:then_0
      ;[1 1 1] Set input System
      (bind _asplayer_controller (Utilities|Casting|CastToPlayerController (Pawn|GetController)))
      (Utilities|IsValid (PlayerController|LocalPlayerSubsystems|GetEnhancedInputLocalPlayerSubsystem _asplayer_controller)
        (:Is%20Valid
          (Input|AddMappingContext (PlayerController|LocalPlayerSubsystems|GetEnhancedInputLocalPlayerSubsystem _asplayer_controller) "/Game/TheRite_Content/Input/Alex_InputContext.Alex_InputContext" 0 "(bIgnoreAllPressedKeysUntilRelease=True,bForceImmediately=False)"))))
    (:then_1
      ;[1 1 1] Show Widget
      (bind _returnvalue (UserInterface|CreateWidget "/Game/TheRite_Content/Ui/WBP_Paused.WBP_Paused_C"))
      (bind _output_get (Variables|Default|SetPuaseMenu _returnvalue))
      (UserInterface|Viewport|AddtoViewport _output_get 0)
      (Widget|SetVisibility _output_get "Hidden")
      (bind _returnvalue_2 (UserInterface|CreateWidget "/Game/TheRite_Content/Ui/UI_CenterDot.UI_CenterDot_C"))
      (bind _output_get_2 (Variables|Default|SetUI_CenterDot _returnvalue_2))
      (UserInterface|Viewport|AddtoViewport _output_get_2 0))
    (:then_2
      ;[1 1 1] Comment
      (Rendering|SetVisibility (Variables|Default|GetPointLight) false false))
    (:then_3
      (EventDispatchers|BindEventtoLighterMonatge (delegate Custom|Montage%20Animation%20On%20Off)))))

(event EventTick
  (params (DeltaSeconds :type Float%20%28single-precision%29))
  (Utilities|FlowControl|Sequence
    (:then_0
      ;[1 1 1] Check Ligher Coold Down
      (CallFunction|CheckLighterCooldDown DeltaSeconds))
    (:then_1
      (if (== (Utilities|Array|Length (Variables|Interactions|GetItemsPickables)) 0)
        (Default|CallOnAllItemsCollected)))
    (:then_2
      (CallFunction|HeadBob))
    (:then_3
      (CallFunction|Breath DeltaSeconds))
    (:then_4
      (bind _output_get (Variables|Sound|SetAudio%20Timer (+ DeltaSeconds (Variables|Sound|GetAudio%20Timer))))
      (if (>= _output_get 2.05)
        (Variables|Sound|SetcanSound true)
        (Variables|Sound|SetAudio%20Timer 0.0)))
    (:then_5
      (CallFunction|LineTraces))))

(fn ConstructionScript)

(fn StartSprint
  (Variables|/Script/Engine.CharacterMovementComponent|SetMaxWalkSpeed (Variables|Character|GetCharacterMovement) (Variables|Movement|GetRunSpeed)))

(fn StopSprint
  (Variables|/Script/Engine.CharacterMovementComponent|SetMaxWalkSpeed (Variables|Character|GetCharacterMovement) (Variables|Movement|GetWalkSpedd)))

(fn SetInteraction
  (params (interaaction :type Boolean) (Interactuable :type I%20Interactuable%20Interface)))

(fn CheckLighterON
  (bind _pointlight (Variables|Default|GetPointLight))
  (if (not (Variables|Flashlight|GetFlashlight))
    (if (Variables|Flashlight|GetFlashLighOnCD)
      (if (Variables|Sound|GetcanSound)
        (Audio|SpawnSoundatLocation (Variables|Sound|GetSound) (Transformation|GetActorLocation) "0, 0, 0" 1.0 1.0 0.0 0 0)
        (Variables|Sound|SetcanSound false)
        (Variables|Flashlight|SetFlashlight false :!label _label)
        (Rendering|SetVisibility _pointlight false false)
        (Default|CallLighterMonatge :!label _label_2))
      (else
        (Audio|SpawnSoundatLocation "/Game/TheRite_Content/Sound/SoundFX/SFX_LighterOn.SFX_LighterOn" "0, 0, 0" "0, 0, 0" 1.0 1.0 -1.0 0 0)
        (Variables|Flashlight|SetFlashlight true)
        (Rendering|SetVisibility _pointlight true false)
        (goto _label_2)))
    (else
      (goto _label))))

(fn CheckLighterCooldDown
  (params (deltaSeconds :type Float%20%28double-precision%29))
  (if (Variables|Flashlight|GetFlashLighOnCD)
    (Variables|Flashlight|SetFlashLightCd_Timer (+ (Variables|Flashlight|GetFlashLightCd_Timer) deltaSeconds))
    (if (>= (Variables|Flashlight|GetFlashLightCd_Timer) (Variables|Flashlight|GetFlashLightCd))
      (Variables|Flashlight|SetFlashLightCd_Timer 0.0)
      (Variables|Flashlight|SetFlashLighOnCD false)
      (elif (<= (Variables|Flashlight|GetFlashLightTimer) 0.0)
        (Variables|Flashlight|SetFlashLightTimer 0.0)
        (else
          (Variables|Flashlight|SetFlashLightTimer (- (Variables|Flashlight|GetFlashLightTimer) deltaSeconds)))))
    (elif (Variables|Flashlight|GetFlashlight)
      (bind _output_get (Variables|Flashlight|SetFlashLightTimer (+ deltaSeconds (Variables|Flashlight|GetFlashLightTimer))))
      (if (>= _output_get (Variables|Flashlight|GetMaxLighterTime))
        (Variables|Flashlight|SetFlashlight false)
        (Rendering|SetVisibility (Variables|Default|GetPointLight) false false)
        (Variables|Flashlight|SetFlashLighOnCD true)
        (Default|CallLighterMonatge))
      (elif (<= (Variables|Flashlight|GetFlashLightTimer) 0.0)
        (Variables|Flashlight|SetFlashLightTimer 0.0)
        (else
          (Variables|Flashlight|SetFlashLightTimer (- (Variables|Flashlight|GetFlashLightTimer) deltaSeconds)))))))

(fn ObteinMainItem
  (params (Item%20Name :type String))
  (bind _itemspickables (Variables|Interactions|GetItemsPickables))
  (for (_array_element _array_index) _itemspickables
    (if (Utilities|Enum|Equal(Enum) (.name (Utilities|Array|Get(acopy) _itemspickables _array_index)) Item%20Name)
      (Utilities|Array|SetArrayElem (Variables|Interactions|GetItemsPickables) _array_index (Utilities|Struct|MakeItemPickable "" true))
      (Utilities|Array|RemoveItem _itemspickables _array_element))))

(fn FlickingLighter
  (params (On :type Boolean))
  (bind _pointlight (Variables|Default|GetPointLight))
  (if On
    (Rendering|Components|Light|SetLightFunctionMaterial _pointlight (Variables|Flashlight|GetAggresive%20Material))
    (Development|PrintString "On")
    (else
      (Rendering|Components|Light|SetLightFunctionMaterial _pointlight (Variables|Flashlight|GetNormal%20Material))
      (Development|PrintString "Off"))))

(fn Breath
  (params (DeltaTime :type Float%20%28double-precision%29))
  (if (> (Variables|Sound|GetBreathTimer) 15.0)
    (Audio|PlaySound2D "/Game/TheRite_Content/Sound/SoundCue/BreathCue.BreathCue" 3.0 1.0 0.0 0 0 false)
    (Variables|Sound|SetBreathTimer 0.0)
    (else
      (Variables|Sound|SetBreathTimer (+ DeltaTime (Variables|Sound|GetBreathTimer))))))

(fn LineTraces
  (bind _ui_centerdot (Variables|Default|GetUI_CenterDot))
  (bind _camera (Variables|Default|GetCamera))
  (bind _returnvalue (Transformation|GetWorldLocation _camera))
  (bind _outhit (Collision|SphereTraceByChannel _returnvalue (+ _returnvalue (* (Math|Vector|GetForwardVector (Transformation|GetWorldRotation _camera)) (Variables|Default|GetRangeInteractuable))) 7.5 "TraceTypeQuery2" false 0 "None" true "(R=1.000000,G=0.000000,B=0.000000,A=1.000000)" "(R=0.000000,G=1.000000,B=0.000000,A=1.000000)" 2.0))
  (bind _asiinteractuable (Utilities|Casting|CastToIInteractuable (.HitActor (Collision|BreakHitResult _outhit)))
    (:then
      (bind _output_get (Variables|Interactions|SetActualnteractuable _asiinteractuable))
      (bind (_lock _isadoor) (CallFunction|CasttoDoor _output_get))
      (if _isadoor
        (if _lock
          (Variables|Interactions|SetCanInteract true)
          (Default|Interacat _ui_centerdot false true)
          (else
            (Variables|Interactions|SetCanInteract true :!label _label)
            (Default|Interacat _ui_centerdot false false)))
        (else
          (bind _asbp_portrait (Utilities|Casting|CastToBP_Portrait _output_get)
            (:then
              (if (Variables|/Game/TheRite_Content/Blueprints/Interactuables/BP_Portrait.BP_Portrait_C|GetPuzzleReady _asbp_portrait)
                (goto _label)))
            (:CastFailed
              (goto _label))))))
    (:CastFailed
      (Variables|Interactions|SetActualnteractuable 0)
      (Variables|Interactions|SetCanInteract false)
      (Default|Interacat _ui_centerdot true false))))

(fn CasttoDoor
  (params (Interactuable :type I%20Interactuable%20Interface))
  (bind _asbp_door (Utilities|Casting|CastToBP_Door Interactuable)
    (:then
      (if (Variables|/Game/TheRite_Content/Blueprints/Interactuables/BP_Door.BP_Door_C|GetIsLocked _asbp_door)
        _
        (elif (Variables|/Game/TheRite_Content/Blueprints/Interactuables/BP_Door.BP_Door_C|GetNeedKey _asbp_door)
          (if (Variables|/Game/TheRite_Content/Blueprints/Interactuables/BP_Door.BP_Door_C|GetKeyUnlocked _asbp_door)
            (return false true)
            (else
              _))
          (else
            (return false true))))
      (return true true))
    (:CastFailed
      (return false false))))