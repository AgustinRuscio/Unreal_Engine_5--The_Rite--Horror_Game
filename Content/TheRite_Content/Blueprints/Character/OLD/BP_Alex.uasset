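; BP_Alex is the first-person player character for a horror game, with sprint, lighter, hint, pause menu and jumpscare handling.
; BP_Controller dispatchers drive its input events.
; Tick runs speed-based camera shakes, periodic breathing, the lighter's burn and cooldown timers, and a camera sphere trace for IInteractuable actors.
; Interacting plays the target's voice clip and calls its Interaction, with tracing and further interaction blocked until the audio finishes.
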(event Custom|Montage%20Animation%20On%20Off
  (bind _lighter (Variables|Default|GetLighter))
  (if (Variables|Flashlight|GetFlashlight)
    (Animation|PlayAnimMontage "/Game/TheRite_Content/Art/Models/Alex/NewModel/A_Lighter_Montage.A_Lighter_Montage" 1.0 "None")
    (Rendering|SetVisibility _lighter true false)
    (else
      (Animation|StopAnimMontage "/Game/TheRite_Content/Art/Models/Alex/NewModel/A_Lighter_Montage.A_Lighter_Montage")
      (Rendering|SetVisibility _lighter false false))))

(event Custom|HeadBob
  (bind _returnvalue (Game|GetPlayerController 0))
  (bind _returnvalue_2 (Transformation|GetVelocity))
  (bind _returnvalue_3 (Math|Vector|VectorLength _returnvalue_2))
  ;[1 1 1] HeadBob
  (if (> _returnvalue_3 0.0)
    (if (< _returnvalue_3 7e+02)
      (Game|Feedback|ClientStartCameraShake _returnvalue "/Game/TheRite_Content/Blueprints/Others/CameraShake/CameraShake_Walk.CameraShake_Walk_C" 1.0 "CameraLocal" "0, 0, 0")
      (else
        (Game|Feedback|ClientStartCameraShake _returnvalue "/Game/TheRite_Content/Blueprints/Others/CameraShake/CameraShake_Run.CameraShake_Run_C" 1.0 "CameraLocal" "0, 0, 0")))
    (else
      (Game|Feedback|ClientStartCameraShake _returnvalue "/Game/TheRite_Content/Blueprints/Others/CameraShake/CameraShake_Idle.CameraShake_Idle_C" 1.0 "CameraLocal" "0, 0, 0"))))

(event Custom|Move%20Alex
  (params (X :type Float%20%28double-precision%29) (Y :type Float%20%28double-precision%29))
  ;[1 1 1] Inputs
  ;;[1 1 1] Move Character
  (Pawn|Input|AddMovementInput (Transformation|GetActorRightVector) X false)
  (Pawn|Input|AddMovementInput (Transformation|GetActorForwardVector) Y false))

(event Custom|CheckHolding
  (params (IsHolding :type Boolean))
  ;[1 1 1] Inputs
  ;;[1 0 0] Use interactuable
  (Variables|Default|SetHoldingInteractBTN IsHolding))

(event Custom|Interaction
  ;[1 1 1] Inputs
  ;;[1 0 0] Use interactuable
  (if (and (Variables|Default|GetCanTalk) (Variables|Interactions|GetCanInteract))
    (Utilities|IsValid (Variables|Default|GetSoundBase)
      (:Is%20Valid
        (CallFunction|PlaySound))
      (:Is%20Not%20Valid
        _))
    (Default|Interaction (Variables|Interactions|GetActualnteractuable))))

(event Custom|Move%20Camera
  (params (X :type Float%20%28double-precision%29) (Y :type Float%20%28double-precision%29) (Door%20Float :type Float%20%28double-precision%29))
  ;[1 1 1] Inputs
  ;;[1 1 1] Move Camera
  (Pawn|Input|AddControllerYawInput X)
  (Pawn|Input|AddControllerPitchInput Y)
  (Variables|Default|SetDoorFloat Door%20Float))

(event Custom|Close%20hint
  ;[1 1 1] Inputs
  ;;[1 1 1] Open Hints
  (if (Variables|Default|GetHasHint)
    (Animation|StopAnimMontage "/Game/TheRite_Content/Art/Models/Alex/NewModel/A_Hint_Alex_Montage.A_Hint_Alex_Montage")
    (Rendering|SetVisibility (Variables|Default|GetHint) false false)))

(event Custom|Open%20Hint
  ;[1 1 1] Inputs
  ;;[1 1 1] Open Hints
  (if (Variables|Default|GetHasHint)
    (Animation|PlayAnimMontage "/Game/TheRite_Content/Art/Models/Alex/NewModel/A_Hint_Alex_Montage.A_Hint_Alex_Montage" 1.0 "None")
    (Rendering|SetVisibility (Variables|Default|GetHint) true false)))

(event Custom|Play%20Sound
  ;[1 1 1] Talk System
  (Variables|Default|SetCanTalk false)
  (bind _returnvalue (Audio|SpawnSound2D (Variables|Default|GetSoundBase) 1.0 1.0 0.0 0))
  (EventDispatchers|BindEventtoOnAudioFinished _returnvalue (delegate Custom|OnAudioFinish)))

(event Custom|OpenPause
  (bind _returnvalue (Game|GetPlayerController 0))
  (bind _puasemenu (Variables|Default|GetPuaseMenu))
  ;[1 1 1] Inputs
  ;;[1 1 1] Puase game
  (Utilities|FlowControl|FlipFlop
    (:A
      (Widget|SetVisibility _puasemenu "Visible")
      (Game|SetGamePaused true)
      (Variables|/Script/Engine.PlayerController|SetbShowMouseCursor _returnvalue true))
    (:B
      (Widget|SetVisibility _puasemenu "Hidden")
      (Game|SetGamePaused false)
      (Variables|/Script/Engine.PlayerController|SetbShowMouseCursor _returnvalue false))))

(event Custom|Camera%20Targetting
  (params (Target :type Vector))
  ;[1 1 1] Make camera focus on a Target
  (Timeline|Timeline PlayFromStart
    (:Update
      (Pawn|SetControlRotation (Game|GetPlayerController 0) (Math|Interpolation|RInterpTo (Pawn|GetControlRotation :!class /Script/Engine.Pawn) (Math|Rotator|FindLookatRotation (Transformation|GetActorLocation) Target) (Utilities|Time|GetWorldDeltaSeconds) 2.0)))))

(event Custom|ForceTalk
  (params (Sould :type Sound%20Base%20Object%20Reference))
  ;[1 1 1] Talk System
  (if (Variables|Default|GetCanTalk)
    _
    (else
      (CallFunction|StopAudio)))
  (Variables|Default|SetSoundBase Sould)
  (CallFunction|PlaySound))

(event Custom|OnAudioFinish
  ;[1 1 1] Talk System
  (Variables|Default|SetCanTalk true))

(event Custom|Stop%20Audio
  ;[1 1 1] Talk System
  (Audio|Components|Audio|Stop (stale Custom|Play%20Sound _returnvalue)))

(event Custom|OnJumpScare
  (bind _tiffanyscreammer (Variables|Default|GetTiffanyscreammer))
  (Input|DisableInput 0)
  (Rendering|SetVisibility _tiffanyscreammer true false)
  (Animation|Montage|PlayMontage _tiffanyscreammer "/Game/TheRite_Content/Art/Models/Tiffany/NewTiffany/TiffanyScream_Montage.TiffanyScream_Montage"
    (:OnCompleted
      _)
    (:OnInterrupted
      _))
  (Rendering|SetVisibility (Variables|Default|GetTiffanyscreammer) false false)
  (Input|EnableInput 0))

(event Custom|BindActions
  (bind _asbp_controller (Utilities|Casting|CastToBP_Controller (Game|GetPlayerController 0))
    (:then
      (bind _output_get (Variables|Default|SetAs%20BP%20Controller _asbp_controller))
      (EventDispatchers|BindEventtoStartSprint _output_get (EventDispatchers|CreateEvent :!event StartSprint))
      (EventDispatchers|BindEventtoStopSprint _output_get (EventDispatchers|CreateEvent :!event StopSprint))
      (EventDispatchers|BindEventtoTurnLighteron (Variables|Default|GetAs%20BP%20Controller) (EventDispatchers|CreateEvent :!event Custom|TurnLighterIfPosible))
      (EventDispatchers|BindEventtoMovePlayer (Variables|Default|GetAs%20BP%20Controller) (EventDispatchers|CreateEvent :!event Custom|Move%20Alex))
      (EventDispatchers|BindEventtoInteractionPress (Variables|Default|GetAs%20BP%20Controller) (EventDispatchers|CreateEvent :!event Custom|Interaction))
      (EventDispatchers|BindEventtoHoldingBTN (Variables|Default|GetAs%20BP%20Controller) (EventDispatchers|CreateEvent :!event Custom|CheckHolding))
      (EventDispatchers|BindEventtoMoveCamera (Variables|Default|GetAs%20BP%20Controller) (EventDispatchers|CreateEvent :!event Custom|Move%20Camera))
      (EventDispatchers|BindEventtoOpenHint (Variables|Default|GetAs%20BP%20Controller) (EventDispatchers|CreateEvent :!event Custom|Open%20Hint))
      (EventDispatchers|BindEventtoCloseHint (Variables|Default|GetAs%20BP%20Controller) (EventDispatchers|CreateEvent :!event Custom|Close%20hint))
      (EventDispatchers|BindEventtoPaused (Variables|Default|GetAs%20BP%20Controller) (EventDispatchers|CreateEvent :!event Custom|OpenPause)))
    (:CastFailed
      (Development|PrintString "No es el controller propio"))))

(event Custom|TurnLighterIfPosible
  ;[1 1 1] Inputs
  ;;[1 1 1] Turn on Lighter (if possible)
  (if (Variables|Default|GetCanUseFlashLight)
    (CallFunction|CheckLighterON)))

(event EventBeginPlay
  (Utilities|FlowControl|Sequence
    (:then_0
      (CallFunction|BindActions))
    (:then_1
      ;[1 1 1] Show Widget
      (bind _returnvalue (UserInterface|CreateWidget "/Game/TheRite_Content/Ui/WBP_Paused.WBP_Paused_C"))
      (bind _output_get (Variables|Default|SetPuaseMenu _returnvalue))
      (UserInterface|Viewport|AddtoViewport _output_get 0)
      (Widget|SetVisibility _output_get "Hidden")
      (bind _returnvalue_2 (UserInterface|CreateWidget "/Game/TheRite_Content/Ui/UI_CenterDot.UI_CenterDot_C"))
      (bind _output_get_2 (Variables|Default|SetUI_CenterDot _returnvalue_2))
      (UserInterface|Viewport|AddtoViewport _output_get_2 0))
    (:then_2
      ;[1 1 1] Comment
      (Rendering|SetVisibility (Variables|Default|GetPointLight) false false))
    (:then_3
      (EventDispatchers|BindEventtoLighterMonatge (delegate Custom|Montage%20Animation%20On%20Off)))))

(event EventTick
  (params (DeltaSeconds :type Float%20%28single-precision%29))
  (Utilities|FlowControl|Sequence
    (:then_0
      ;[1 1 1] Check Ligher Coold Down
      (CallFunction|CheckLighterCooldDown DeltaSeconds))
    (:then_1)
    (:then_2
      (CallFunction|HeadBob))
    (:then_3
      (CallFunction|Breath DeltaSeconds))
    (:then_4
      (bind _output_get (Variables|Sound|SetAudio%20Timer (+ DeltaSeconds (Variables|Sound|GetAudio%20Timer))))
      (if (>= _output_get 2.05)
        (Variables|Sound|SetcanSound true)
        (Variables|Sound|SetAudio%20Timer 0.0)))
    (:then_5
      (CallFunction|LineTraces))))

(fn ConstructionScript)

(fn StartSprint
  (Variables|/Script/Engine.CharacterMovementComponent|SetMaxWalkSpeed (Variables|Character|GetCharacterMovement) (Variables|Movement|GetRunSpeed)))

(fn StopSprint
  (Variables|/Script/Engine.CharacterMovementComponent|SetMaxWalkSpeed (Variables|Character|GetCharacterMovement) (Variables|Movement|GetWalkSpedd)))

(fn SetInteraction
  (params (interaaction :type Boolean) (Interactuable :type I%20Interactuable%20Interface)))

(fn CheckLighterON
  (bind _pointlight (Variables|Default|GetPointLight))
  (if (not (Variables|Flashlight|GetFlashlight))
    (if (Variables|Flashlight|GetFlashLighOnCD)
      (if (Variables|Sound|GetcanSound)
        (Audio|SpawnSoundatLocation (Variables|Sound|GetSound) (Transformation|GetActorLocation) "0, 0, 0" 1.0 1.0 0.0 0 0)
        (Variables|Sound|SetcanSound false)
        (Variables|Flashlight|SetFlashlight false :!label _label)
        (Rendering|SetVisibility _pointlight false false)
        (Default|CallLighterMonatge :!label _label_2))
      (else
        (Audio|SpawnSoundatLocation "/Game/TheRite_Content/Sound/SoundFX/SFX_LighterOn.SFX_LighterOn" "0, 0, 0" "0, 0, 0" 1.0 1.0 -1.0 0 0)
        (Variables|Flashlight|SetFlashlight true)
        (Rendering|SetVisibility _pointlight true false)
        (goto _label_2)))
    (else
      (goto _label))))

(fn CheckLighterCooldDown
  (params (deltaSeconds :type Float%20%28double-precision%29))
  (if (Variables|Flashlight|GetFlashLighOnCD)
    (Variables|Flashlight|SetFlashLightCd_Timer (+ (Variables|Flashlight|GetFlashLightCd_Timer) deltaSeconds))
    (if (>= (Variables|Flashlight|GetFlashLightCd_Timer) (Variables|Flashlight|GetFlashLightCd))
      (Variables|Flashlight|SetFlashLightCd_Timer 0.0)
      (Variables|Flashlight|SetFlashLighOnCD false)
      (elif (<= (Variables|Flashlight|GetFlashLightTimer) 0.0)
        (Variables|Flashlight|SetFlashLightTimer 0.0)
        (else
          (Variables|Flashlight|SetFlashLightTimer (- (Variables|Flashlight|GetFlashLightTimer) deltaSeconds)))))
    (elif (Variables|Flashlight|GetFlashlight)
      (bind _output_get (Variables|Flashlight|SetFlashLightTimer (+ deltaSeconds (Variables|Flashlight|GetFlashLightTimer))))
      (if (>= _output_get (Variables|Flashlight|GetMaxLighterTime))
        (Variables|Flashlight|SetFlashlight false)
        (Rendering|SetVisibility (Variables|Default|GetPointLight) false false)
        (Variables|Flashlight|SetFlashLighOnCD true)
        (Default|CallLighterMonatge))
      (elif (<= (Variables|Flashlight|GetFlashLightTimer) 0.0)
        (Variables|Flashlight|SetFlashLightTimer 0.0)
        (else
          (Variables|Flashlight|SetFlashLightTimer (- (Variables|Flashlight|GetFlashLightTimer) deltaSeconds)))))))

(fn ObteinMainItem
  (params (Item%20Name :type String))
  (bind _itemspickables (Variables|Interactions|GetItemsPickables))
  (for (_array_element _array_index) _itemspickables
    (if (Utilities|Enum|Equal(Enum) (.name (Utilities|Array|Get(acopy) _itemspickables _array_index)) Item%20Name)
      (Utilities|Array|SetArrayElem (Variables|Interactions|GetItemsPickables) _array_index (Utilities|Struct|MakeItemPickable "" true))
      (Utilities|Array|RemoveItem _itemspickables _array_element))))

(fn FlickingLighter
  (params (On :type Boolean))
  (bind _pointlight (Variables|Default|GetPointLight))
  (if On
    (Rendering|Components|Light|SetLightFunctionMaterial _pointlight (Variables|Flashlight|GetAggresive%20Material))
    (else
      (Rendering|Components|Light|SetLightFunctionMaterial _pointlight (Variables|Flashlight|GetNormal%20Material)))))

(fn Breath
  (params (DeltaTime :type Float%20%28double-precision%29))
  (if (> (Variables|Sound|GetBreathTimer) 15.0)
    (Audio|PlaySound2D "/Game/TheRite_Content/Sound/SoundCue/BreathCue.BreathCue" 3.0 1.0 0.0 0 0 false)
    (Variables|Sound|SetBreathTimer 0.0)
    (else
      (Variables|Sound|SetBreathTimer (+ DeltaTime (Variables|Sound|GetBreathTimer))))))

(fn LineTraces
  (bind _camera (Variables|Default|GetCamera))
  (bind _returnvalue (Transformation|GetWorldLocation _camera))
  (if (Variables|Default|GetCanTalk)
    (bind _outhit (Collision|SphereTraceByChannel _returnvalue (+ _returnvalue (* (Math|Vector|GetForwardVector (Transformation|GetWorldRotation _camera)) (Variables|Default|GetRangeInteractuable))) 7.5 "TraceTypeQuery2" false 0 "None" true "(R=1.000000,G=0.000000,B=0.000000,A=1.000000)" "(R=0.000000,G=1.000000,B=0.000000,A=1.000000)" 2.0))
    (bind _asiinteractuable (Utilities|Casting|CastToIInteractuable (.HitActor (Collision|BreakHitResult _outhit)))
      (:then
        (bind _output_get (Variables|Interactions|SetActualnteractuable _asiinteractuable))
        (bind _sound (Default|GetSound _output_get))
        (Variables|Default|SetSoundBase _sound)
        (bind (_lock _isadoor) (CallFunction|CasttoDoor _output_get))
        (if _isadoor
          (if _lock
            (Variables|Interactions|SetCanInteract true)
            (else
              (Variables|Interactions|SetCanInteract true :!label _label)))
          (else
            (goto _label))))
      (:CastFailed
        (Variables|Interactions|SetActualnteractuable 0)
        (Variables|Default|SetSoundBase 0)
        (Variables|Interactions|SetCanInteract false)))))

(fn CasttoDoor
  (params (Interactuable :type I%20Interactuable%20Interface))
  (bind _asbp_door (Utilities|Casting|CastToBP_Door Interactuable)
    (:then
      (if (Variables|/Game/TheRite_Content/Blueprints/Interactuables/Old/BP_Door.BP_Door_C|GetIsLocked _asbp_door)
        _
        (elif (Variables|/Game/TheRite_Content/Blueprints/Interactuables/Old/BP_Door.BP_Door_C|GetNeedKey _asbp_door)
          (if (Variables|/Game/TheRite_Content/Blueprints/Interactuables/Old/BP_Door.BP_Door_C|GetKeyUnlocked _asbp_door)
            (return false true)
            (else
              _))
          (else
            (return false true))))
      (return true true))
    (:CastFailed
      (return false false))))