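; BP_Tiffany is an AI-driven character whose proximity disturbs nearby lights and the lighter carried by BP_Alex.
; StartMovement flags her as walking and writes the target and a bool to her controller's Blackboard.
; Sphere overlaps search for nearby BP_Light actors, switching them between aggressive and normal materials and toggling Alex's lighter flicker.
; Setter functions store waypoints and configure mesh visibility, capsule collision and whether she has to move.
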(event OnComponentBeginOverlap(Sphere)
  (params (OverlappedComponent :type Primitive%20Component%20Object%20Reference) (OtherActor :type Actor%20Object%20Reference) (OtherComp :type Primitive%20Component%20Object%20Reference) (OtherBodyIndex :type Integer) (bFromSweep :type Boolean) (SweepResult :type Hit%20Result%20Structure%20%28by%20ref%29))
  (bind (_outactors _returnvalue) (Collision|SphereOverlapActors (Transformation|GetActorLocation) 5e+02 (Utilities|Array|MakeArray "ObjectTypeQuery2") "/Game/TheRite_Content/Blueprints/Others/BP_Light.BP_Light_C"))
  (if _returnvalue
    (for _array_element _outactors
      (Default|AggresiveMaterial (.AsBP%20Light (Utilities|Casting|CastToBP_Light _array_element)))
      (bind _asbp_alex (Utilities|Casting|CastToBP_Alex OtherActor))
      (Default|FlickingLighter _asbp_alex true))
    (else
      (bind _asbp_alex_2 (Utilities|Casting|CastToBP_Alex OtherActor))
      (Default|FlickingLighter _asbp_alex_2 true))))

(event OnComponentEndOverlap(Sphere)
  (params (OverlappedComponent :type Primitive%20Component%20Object%20Reference) (OtherActor :type Actor%20Object%20Reference) (OtherComp :type Primitive%20Component%20Object%20Reference) (OtherBodyIndex :type Integer))
  (bind (_outactors _returnvalue) (Collision|SphereOverlapActors (Transformation|GetActorLocation) 5e+02 (Utilities|Array|MakeArray "ObjectTypeQuery2") "/Game/TheRite_Content/Blueprints/Others/BP_Light.BP_Light_C"))
  (if _returnvalue
    (for _array_element _outactors
      (Default|NormalMaterial (.AsBP%20Light (Utilities|Casting|CastToBP_Light _array_element)))
      (bind _asbp_alex (Utilities|Casting|CastToBP_Alex OtherActor))
      (Default|FlickingLighter _asbp_alex false))
    (else
      (bind _asbp_alex_2 (Utilities|Casting|CastToBP_Alex OtherActor))
      (Default|FlickingLighter _asbp_alex_2 false))))

(event Custom|StartMovement
  (params (New%20Target :type Target%20Point%20Object%20Reference))
  (bind _returnvalue (Pawn|GetController))
  (bind _returnvalue_2 (AI|GetBlackboard _returnvalue))
  (Variables|Default|SetWalking true)
  (AI|Components|Blackboard|SetValueasObject _returnvalue_2 (Variables|Default|GetTargetKey) New%20Target)
  (AI|Components|Blackboard|SetValueasBool _returnvalue_2 (Variables|Default|GetBooleanKey) true))

(fn ConstructionScript)

(fn SetWaypoints
  (params (NewParam :type Array%20of%20Target%20Point%20Object%20References))
  (Variables|Default|SetWaypoits NewParam))

(fn SetData
  (params (IsVisible :type Boolean) (NoCollision :type Boolean) (HastToMove :type Boolean))
  (Rendering|SetVisibility (Variables|Character|GetMesh) IsVisible false)
  (if NoCollision
    (Collision|SetCollisionEnabled (Variables|Collision|GetCapsuleComponent) "NoCollision"))
  (Variables|Default|SetHasToMove HastToMove))