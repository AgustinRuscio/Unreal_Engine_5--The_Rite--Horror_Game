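; BP_xd is a one-shot trigger that briefly blacks out the lights in its XDDD array when BP_AlexPlus enters its box.
; The overlap hides each light component and starts a three-second timer, whose event shows them again and destroys the trigger.
; DoOnce precedes the cast, so any first overlapping actor uses up the trigger.
; The timer and destroy calls sit inside the loop bodies.
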(event OnComponentBeginOverlap(Box)
  (params (OverlappedComponent :type Primitive%20Component%20Object%20Reference) (OtherActor :type Actor%20Object%20Reference) (OtherComp :type Primitive%20Component%20Object%20Reference) (OtherBodyIndex :type Integer) (bFromSweep :type Boolean) (SweepResult :type Hit%20Result%20Structure%20%28by%20ref%29))
  (Utilities|FlowControl|DoOnce false
    (:Completed
      (Utilities|Casting|CastToBP_AlexPlus OtherActor)
      (for _array_element (Variables|Default|GetXDDD)
        (Rendering|SetVisibility (Variables|/Script/Engine.Light|GetLightComponent _array_element) false false)
        (Utilities|Time|SetTimerbyEvent (delegate Custom|CustomEvent) 3.0)))))

(event Custom|CustomEvent
  (for _array_element (Variables|Default|GetXDDD)
    (Rendering|SetVisibility (Variables|/Script/Engine.Light|GetLightComponent _array_element) true false)
    (Actor|DestroyActor)))

(event EventBeginPlay)

(event Collision|EventActorBeginOverlap
  (params (OtherActor :type Actor%20Object%20Reference)))

(event EventTick
  (params (DeltaSeconds :type Float%20%28single-precision%29)))

(fn ConstructionScript)