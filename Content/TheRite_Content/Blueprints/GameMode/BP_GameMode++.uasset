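; BP_GameMode++ is a game mode Blueprint that handles achievement unlocks by name for the first player controller.
; Its UnlockAchievemetns event caches achievements, then looks up the cached progress for the given ID.
; It writes progress only when the ID exists with no progress above zero, printing debug messages for already unlocked, missing ID or failed caching.
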(event EventUnlockAchievemetns
  (params (unlockName :type Name :default "None"))
  (bind _returnvalue (Game|GetPlayerController 0))
  (|CacheAchievements _returnvalue _returnvalue
    (:OnSuccess
      (bind (_bfoundid _progress) (Class|AchievementBlueprintLibrary|GetCachedAchievementProgress (Game|GetPlayerController 0) unlockName))
      (if _bfoundid
        (if (> _progress 0.0)
          (Development|PrintString "Already unlocked")
          (else
            (|WriteProgress (Game|GetPlayerController 0) (Utilities|String|ToString(Name) unlockName) 1e+02)))
        (else
          (Development|PrintString "Didint find ID"))))
    (:OnFailure
      (Development|PrintString "Couldnt Cache"))))

(fn ConstructionScript)