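; BP_Controller is the player controller for TheRite, turning Enhanced Input actions into gameplay signals.
; On BeginPlay it adds the Alex_InputContext mapping context.
; Each action calls an event dispatcher for sprint, lighter, movement, camera, interaction, hints or pause, leaving the behavior to whatever binds to it.
; Interaction separates press from hold, with completion also firing the hold signal, and releasing or canceling LeaveFocus closes hints.
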(event Input|EnhancedActionEvents|EnhancedInputActionAlex_Look
  (params (ActionValue :type Vector%202D%20Structure) (ElapsedSeconds :type Float%20%28double-precision%29) (TriggeredSeconds :type Float%20%28double-precision%29) (InputAction :type Input%20Action%20Object%20Reference :default "/Game/TheRite_Content/Input/Input_Actions/Alex_Look.Alex_Look"))
  ;[1 1 1] Inputs
  ;;[1 1 1] Move Camera
  (:Triggered
    (Default|CallMoveCamera (.x ActionValue) (.y ActionValue) (.x ActionValue))))

(event Input|EnhancedActionEvents|EnhancedInputActionAlex_Move
  (params (ActionValue :type Vector%202D%20Structure) (ElapsedSeconds :type Float%20%28double-precision%29) (TriggeredSeconds :type Float%20%28double-precision%29) (InputAction :type Input%20Action%20Object%20Reference :default "/Game/TheRite_Content/Input/Input_Actions/Alex_Move.Alex_Move"))
  ;[1 1 1] Inputs
  ;;[1 1 1] Move Character
  (:Triggered
    (Default|CallMovePlayer (.x ActionValue) (.y ActionValue))))

(event Input|EnhancedActionEvents|EnhancedInputActionAlex_Spint
  (params (ActionValue :type Boolean) (ElapsedSeconds :type Float%20%28double-precision%29) (TriggeredSeconds :type Float%20%28double-precision%29) (InputAction :type Input%20Action%20Object%20Reference :default "/Game/TheRite_Content/Input/Input_Actions/Alex_Spint.Alex_Spint"))
  ;[1 1 1] Inputs
  ;;[1 1 1] Sprint
  (:Triggered
    (Default|CallStartSprint))
  (:Completed
    (Default|CallStopSprint)))

(event Input|EnhancedActionEvents|EnhancedInputActionAlex_Interaction
  (params (ActionValue :type Boolean) (ElapsedSeconds :type Float%20%28double-precision%29) (TriggeredSeconds :type Float%20%28double-precision%29) (InputAction :type Input%20Action%20Object%20Reference :default "/Game/TheRite_Content/Input/Input_Actions/Alex_Interaction.Alex_Interaction"))
  ;[1 1 1] Inputs
  ;;[1 0 0] Use interactuable
  (:Triggered
    (Default|CallHoldingBTN ActionValue :!label _label))
  (:Started
    (Default|CallInteractionPress))
  (:Completed
    (goto _label)))

(event Input|EnhancedActionEvents|EnhancedInputActionAlex_Flashlight
  (params (ActionValue :type Boolean) (ElapsedSeconds :type Float%20%28double-precision%29) (TriggeredSeconds :type Float%20%28double-precision%29) (InputAction :type Input%20Action%20Object%20Reference :default "/Game/TheRite_Content/Input/Input_Actions/Alex_Flashlight.Alex_Flashlight"))
  ;[1 1 1] Inputs
  ;;[1 1 1] Turn on Lighter (if possible)
  (:Started
    (Default|CallTurnLighteron)))

(event Input|EnhancedActionEvents|EnhancedInputActionAlex_LeaveFocus
  (params (ActionValue :type Boolean) (ElapsedSeconds :type Float%20%28double-precision%29) (TriggeredSeconds :type Float%20%28double-precision%29) (InputAction :type Input%20Action%20Object%20Reference :default "/Game/TheRite_Content/Input/Input_Actions/Alex_LeaveFocus.Alex_LeaveFocus"))
  ;[1 1 1] Inputs
  ;;[1 1 1] Open Hints
  (:Triggered
    (Default|CallOpenHint))
  (:Canceled
    (Default|CallCloseHint :!label _label))
  (:Completed
    (goto _label)))

(event Input|EnhancedActionEvents|EnhancedInputActionAlex_Pause
  (params (ActionValue :type Boolean) (ElapsedSeconds :type Float%20%28double-precision%29) (TriggeredSeconds :type Float%20%28double-precision%29) (InputAction :type Input%20Action%20Object%20Reference :default "/Game/TheRite_Content/Input/Input_Actions/Alex_Pause.Alex_Pause"))
  ;[1 1 1] Inputs
  ;;[1 1 1] Puase game
  (:Started
    (Default|CallPaused)))

(event EventBeginPlay
  (Input|AddMappingContext (PlayerController|LocalPlayerSubsystems|GetEnhancedInputLocalPlayerSubsystem) "/Game/TheRite_Content/Input/Alex_InputContext.Alex_InputContext" 0 "(bIgnoreAllPressedKeysUntilRelease=True,bForceImmediately=False)"))

(fn ConstructionScript)