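; Player controller for the menu that boots the UI and restores saved settings.
; On BeginPlay it creates a widget stack with UI-only input, then plays the logo sound and pushes the logo screen.
; On first open only, flagged in the GameInstance, it sets shadow and GI quality and loads GameSettings through the GameState.
; It then applies culture and colorblind mode from GameInstance values, with sentinel checks for defaults.
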(event EventBeginPlay
  (CallFunction|CreateVariables)
  (Utilities|FlowControl|Sequence
    (:then_0
      (CallFunction|GetSavedData))
    (:then_1
      (Audio|SpawnSound2D "/Game/TheRite_Content/Sound/LogoSound.LogoSound" 1.0 1.0 0.0 0)
      (Default|PushWidget (Variables|Default|GetMenuStack) "/Game/TheRite_Content/Ui/CommonUI/Widgets/Activables/Menues/WBP_ActivableLogo.WBP_ActivableLogo_C"))))

(fn ConstructionScript)

(fn CreateVariables
  (bind _returnvalue (UserInterface|CreateWidget "/Game/TheRite_Content/Ui/CommonUI/Widgets/Stacks/WBP_MenuStack.WBP_MenuStack_C" self))
  (bind _output_get (Variables|Default|SetMenuStack _returnvalue))
  (Variables|/Game/TheRite_Content/Ui/CommonUI/Widgets/Stacks/WBP_MenuStack.WBP_MenuStack_C|SetPushMenu _output_get false)
  (UserInterface|Viewport|AddtoViewport _output_get 0)
  (Input|SetInputModeUIOnly self (Variables|Default|GetMenuStack) "DoNotLock" true)
  (bind _returnvalue_2 (UserInterface|CreateWidget "/Game/TheRite_Content/Ui/CommonUI/Widgets/Activables/Menues/WBP_ActivableLogo.WBP_ActivableLogo_C" self))
  (Variables|Default|SetActivable%20Logo _returnvalue_2)
  (bind _asbp_game_instance (Utilities|Casting|CastToBP_GameInstance (Game|GetGameInstance)))
  (Variables|Default|SetGame%20Instance _asbp_game_instance))

(fn GetSavedData
  (if (Variables|/Game/TheRite_Content/Blueprints/BP_GameInstance.BP_GameInstance_C|GetFirstOpen (Variables|Default|GetGame%20Instance))
    (bind _returnvalue (Settings|GetGameUserSettings))
    (Class|GameUserSettings|SetShadowQuality _returnvalue 2)
    (Class|GameUserSettings|SetGlobalIlluminationQuality _returnvalue 2)
    (Class|GameUserSettings|ApplySettings _returnvalue false)
    (Variables|/Game/TheRite_Content/Blueprints/BP_GameInstance.BP_GameInstance_C|SetFirstOpen (Variables|Default|GetGame%20Instance) false)
    (CallFunction|Load)))

(fn Load
  (Default|LoadSaveData (.AsGS%20the%20Rite (Utilities|Casting|CastToGS_TheRite (Game|GetGameState))) "GameSettings")
  (CallFunction|LoadCulture)
  (CallFunction|LoadColorblindness))

(fn LoadCulture
  (bind _game_instance (Variables|Default|GetGame%20Instance))
  (bind _currentculture (Variables|/Game/TheRite_Content/Blueprints/BP_GameInstance.BP_GameInstance_C|GetCurrentCulture _game_instance))
  (LocalVariables|SetNewLocalVar_0 (Class|KismetInternationalizationLibrary|GetLocalizedCultures true false false false))
  (if (Utilities|Enum|Equal(Enum) _currentculture "pepe")
    (Class|KismetInternationalizationLibrary|SetCurrentCulture "0")
    (else
      (Class|KismetInternationalizationLibrary|SetCurrentCulture _currentculture))))

(fn LoadColorblindness
  (bind _game_instance (Variables|Default|GetGame%20Instance))
  (LocalVariables|SetColorblindArray (Utilities|Array|MakeArray "NormalVision" "Deuteranope" "Protanope" "Tritanope"))
  (if (== (Variables|/Game/TheRite_Content/Blueprints/BP_GameInstance.BP_GameInstance_C|GetDeficiencyIndex (Variables|Default|GetGame%20Instance)) -2)
    (Class|WidgetBlueprintLibrary|SetColorVisionDeficiencyType "NormalVision" 0.0 false)
    (else
      (Class|WidgetBlueprintLibrary|SetColorVisionDeficiencyType (Variables|/Game/TheRite_Content/Blueprints/BP_GameInstance.BP_GameInstance_C|GetCurrentDeficiency _game_instance) (Variables|/Game/TheRite_Content/Blueprints/BP_GameInstance.BP_GameInstance_C|GetVisionDeficiencySeverity _game_instance) false))))