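; GS_TheRite saves and loads player settings for The Rite: audio volumes, language, color vision deficiency, resolution and gamma.
; SaveGame loads or creates an SG_savegame for the named slot, copies the values from BP_GameInstance, then writes it to disk.
; Loadsavedata reads an existing slot and copies its values back into the game instance, which is cached on BeginPlay.
; It only transfers values and does not apply them.
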(event Custom|SaveGame
  (params (Slot%20Name :type String))
  ;[1 1 1] Save game
  ;;[1 1 1] Save Button
  (Variables|Default|SetSlot%20Name Slot%20Name)
  (bind _returnvalue (SaveGame|DoesSaveGameExist (Variables|Default|GetSlot%20Name)))
  (if _returnvalue
    (bind _returnvalue_2 (SaveGame|LoadGamefromSlot (Variables|Default|GetSlot%20Name)))
    (bind _assg_savegame (Utilities|Casting|CastToSG_savegame _returnvalue_2))
    (bind _output_get (Variables|Default|SetSaveGameRef _assg_savegame))
    (CallFunction|SetSaveDataVariables _output_get)
    (else
      (bind _returnvalue_3 (SaveGame|CreateSaveGameObject "/Game/TheRite_Content/Blueprints/SG_savegame.SG_savegame_C"))
      (bind _output_get_2 (Variables|Default|SetSaveGameRef _returnvalue_3))
      (CallFunction|SetSaveDataVariables _output_get_2))))

(event Custom|LoadValues
  (params (SaveSlot :type SG%20Savegame%20Object%20Reference))
  (bind _as_bp_game_instance (Variables|Default|GetAs%20BP%20Game%20Instance))
  (Variables|/Game/TheRite_Content/Blueprints/BP_GameInstance.BP_GameInstance_C|SetMasterVolumen (Variables|Default|GetAs%20BP%20Game%20Instance) (Variables|/Game/TheRite_Content/Blueprints/SG_savegame.SG_savegame_C|GetMasterVolumen SaveSlot))
  (Variables|/Game/TheRite_Content/Blueprints/BP_GameInstance.BP_GameInstance_C|SetVoiceVolumen (Variables|Default|GetAs%20BP%20Game%20Instance) (Variables|/Game/TheRite_Content/Blueprints/SG_savegame.SG_savegame_C|GetVoiceVolumen (Variables|Default|GetSaveGameRef)))
  (Variables|/Game/TheRite_Content/Blueprints/BP_GameInstance.BP_GameInstance_C|SetMusicVolumen (Variables|Default|GetAs%20BP%20Game%20Instance) (Variables|/Game/TheRite_Content/Blueprints/SG_savegame.SG_savegame_C|GetMusicVolumen (Variables|Default|GetSaveGameRef)))
  (Variables|/Game/TheRite_Content/Blueprints/BP_GameInstance.BP_GameInstance_C|SetFxVolumen (Variables|Default|GetAs%20BP%20Game%20Instance) (Variables|/Game/TheRite_Content/Blueprints/SG_savegame.SG_savegame_C|GetFxVolumen (Variables|Default|GetSaveGameRef)))
  (Variables|/Game/TheRite_Content/Blueprints/BP_GameInstance.BP_GameInstance_C|SetCurrentCulture (Variables|Default|GetAs%20BP%20Game%20Instance) (Variables|/Game/TheRite_Content/Blueprints/SG_savegame.SG_savegame_C|GetCurrentCulture (Variables|Default|GetSaveGameRef)))
  (Variables|/Game/TheRite_Content/Blueprints/BP_GameInstance.BP_GameInstance_C|SetCultureName (Variables|Default|GetAs%20BP%20Game%20Instance) (Variables|/Game/TheRite_Content/Blueprints/SG_savegame.SG_savegame_C|GetCultureName (Variables|Default|GetSaveGameRef)))
  (Variables|/Game/TheRite_Content/Blueprints/BP_GameInstance.BP_GameInstance_C|SetVisionDeficiencySeverity (Variables|Default|GetAs%20BP%20Game%20Instance) (Variables|/Game/TheRite_Content/Blueprints/SG_savegame.SG_savegame_C|GetVisionDeficiencySeverity (Variables|Default|GetSaveGameRef)))
  (Variables|/Game/TheRite_Content/Blueprints/BP_GameInstance.BP_GameInstance_C|SetCurrentDeficiency (Variables|Default|GetAs%20BP%20Game%20Instance) (Variables|/Game/TheRite_Content/Blueprints/SG_savegame.SG_savegame_C|GetCurrentDeficiency (Variables|Default|GetSaveGameRef)))
  (Variables|/Game/TheRite_Content/Blueprints/BP_GameInstance.BP_GameInstance_C|SetDeficiencyIndex _as_bp_game_instance (Variables|/Game/TheRite_Content/Blueprints/SG_savegame.SG_savegame_C|GetDeficencyIndex (Variables|Default|GetSaveGameRef)))
  (Variables|/Game/TheRite_Content/Blueprints/BP_GameInstance.BP_GameInstance_C|SetCultureIndex _as_bp_game_instance (Variables|/Game/TheRite_Content/Blueprints/SG_savegame.SG_savegame_C|Getculturindex (Variables|Default|GetSaveGameRef)))
  (Variables|/Game/TheRite_Content/Blueprints/BP_GameInstance.BP_GameInstance_C|SetResolutionIndex (Variables|Default|GetAs%20BP%20Game%20Instance) (Variables|/Game/TheRite_Content/Blueprints/SG_savegame.SG_savegame_C|GetResolutionIndex (Variables|Default|GetSaveGameRef)))
  (Variables|/Game/TheRite_Content/Blueprints/BP_GameInstance.BP_GameInstance_C|SetGamma (Variables|Default|GetAs%20BP%20Game%20Instance) (Variables|/Game/TheRite_Content/Blueprints/SG_savegame.SG_savegame_C|GetGammaValue (Variables|Default|GetSaveGameRef))))

(event Custom|Load%20save%20data
  (params (slotName :type String))
  (bind _output_get (Variables|Default|SetSlot%20Name slotName))
  (bind _returnvalue (SaveGame|DoesSaveGameExist _output_get))
  (if _returnvalue
    (bind _returnvalue_2 (SaveGame|LoadGamefromSlot (Variables|Default|GetSlot%20Name)))
    (bind _assg_savegame (Utilities|Casting|CastToSG_savegame _returnvalue_2))
    (bind _output_get_2 (Variables|Default|SetSaveGameRef _assg_savegame))
    (CallFunction|LoadValues _output_get_2)))

(event Custom|Set%20Save%20data%20variables
  (params (SaveSlot :type SG%20Savegame%20Object%20Reference))
  ;[1 1 1] Save game
  ;;[1 1 1] Save variables
  (Variables|/Game/TheRite_Content/Blueprints/SG_savegame.SG_savegame_C|SetMasterVolumen SaveSlot (Variables|/Game/TheRite_Content/Blueprints/BP_GameInstance.BP_GameInstance_C|GetMasterVolumen (Variables|Default|GetAs%20BP%20Game%20Instance)))
  (Variables|/Game/TheRite_Content/Blueprints/SG_savegame.SG_savegame_C|SetVoiceVolumen (Variables|Default|GetSaveGameRef) (Variables|/Game/TheRite_Content/Blueprints/BP_GameInstance.BP_GameInstance_C|GetVoiceVolumen (Variables|Default|GetAs%20BP%20Game%20Instance)))
  (Variables|/Game/TheRite_Content/Blueprints/SG_savegame.SG_savegame_C|SetMusicVolumen (Variables|Default|GetSaveGameRef) (Variables|/Game/TheRite_Content/Blueprints/BP_GameInstance.BP_GameInstance_C|GetMusicVolumen (Variables|Default|GetAs%20BP%20Game%20Instance)))
  (Variables|/Game/TheRite_Content/Blueprints/SG_savegame.SG_savegame_C|SetFxVolumen (Variables|Default|GetSaveGameRef) (Variables|/Game/TheRite_Content/Blueprints/BP_GameInstance.BP_GameInstance_C|GetFxVolumen (Variables|Default|GetAs%20BP%20Game%20Instance)))
  (Variables|/Game/TheRite_Content/Blueprints/SG_savegame.SG_savegame_C|SetCurrentCulture (Variables|Default|GetSaveGameRef) (Variables|/Game/TheRite_Content/Blueprints/BP_GameInstance.BP_GameInstance_C|GetCurrentCulture (Variables|Default|GetAs%20BP%20Game%20Instance)))
  (Variables|/Game/TheRite_Content/Blueprints/SG_savegame.SG_savegame_C|SetCultureName (Variables|Default|GetSaveGameRef) (Variables|/Game/TheRite_Content/Blueprints/BP_GameInstance.BP_GameInstance_C|GetCultureName (Variables|Default|GetAs%20BP%20Game%20Instance)))
  (Variables|/Game/TheRite_Content/Blueprints/SG_savegame.SG_savegame_C|SetVisionDeficiencySeverity (Variables|Default|GetSaveGameRef) (Variables|/Game/TheRite_Content/Blueprints/BP_GameInstance.BP_GameInstance_C|GetVisionDeficiencySeverity (Variables|Default|GetAs%20BP%20Game%20Instance)))
  (Variables|/Game/TheRite_Content/Blueprints/SG_savegame.SG_savegame_C|SetCurrentDeficiency (Variables|Default|GetSaveGameRef) (Variables|/Game/TheRite_Content/Blueprints/BP_GameInstance.BP_GameInstance_C|GetCurrentDeficiency (Variables|Default|GetAs%20BP%20Game%20Instance)))
  (Variables|/Game/TheRite_Content/Blueprints/SG_savegame.SG_savegame_C|SetDeficencyIndex (Variables|Default|GetSaveGameRef) (Variables|/Game/TheRite_Content/Blueprints/BP_GameInstance.BP_GameInstance_C|GetDeficiencyIndex (Variables|Default|GetAs%20BP%20Game%20Instance)))
  (Variables|/Game/TheRite_Content/Blueprints/SG_savegame.SG_savegame_C|Setculturindex (Variables|Default|GetSaveGameRef) (Variables|/Game/TheRite_Content/Blueprints/BP_GameInstance.BP_GameInstance_C|GetCultureIndex (Variables|Default|GetAs%20BP%20Game%20Instance)))
  (Variables|/Game/TheRite_Content/Blueprints/SG_savegame.SG_savegame_C|SetResolutionIndex (Variables|Default|GetSaveGameRef) (Variables|/Game/TheRite_Content/Blueprints/BP_GameInstance.BP_GameInstance_C|GetResolutionIndex (Variables|Default|GetAs%20BP%20Game%20Instance)))
  (Variables|/Game/TheRite_Content/Blueprints/SG_savegame.SG_savegame_C|SetGammaValue (Variables|Default|GetSaveGameRef) (Variables|/Game/TheRite_Content/Blueprints/BP_GameInstance.BP_GameInstance_C|GetGamma (Variables|Default|GetAs%20BP%20Game%20Instance)))
  (SaveGame|SaveGametoSlot (Variables|Default|GetSaveGameRef) (Variables|Default|GetSlot%20Name)))

(event EventBeginPlay
  (Variables|Default|SetAs%20BP%20Game%20Instance (.AsBP%20Game%20Instance (Utilities|Casting|CastToBP_GameInstance (Game|GetGameInstance)))))

(fn ConstructionScript)