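; BP_Light is a spotlight actor that can be switched on and off and reacts to Tiffany entering its sphere.
; It stores its starting intensity at BeginPlay so TurnOn can restore it after TurnOff zeroes it.
; A sphere overlap with BP_Tiffany swaps the light function material to an aggressive one.
; A separate NormalMaterial event restores the normal material after a short delay.
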(event OnComponentBeginOverlap(Sphere)
  (params (OverlappedComponent :type Primitive%20Component%20Object%20Reference) (OtherActor :type Actor%20Object%20Reference) (OtherComp :type Primitive%20Component%20Object%20Reference) (OtherBodyIndex :type Integer) (bFromSweep :type Boolean) (SweepResult :type Hit%20Result%20Structure%20%28by%20ref%29))
  (Utilities|Casting|CastToBP_Tiffany OtherActor)
  (CallFunction|AggresiveMaterial))

(event Custom|NormalMaterial
  (Utilities|FlowControl|Delay 2.0)
  (Rendering|Components|Light|SetLightFunctionMaterial (Variables|Default|GetSpotLight) (Variables|Default|GetNormal%20Material)))

(event Custom|AggresiveMaterial
  (Rendering|Components|Light|SetLightFunctionMaterial (Variables|Default|GetSpotLight) (Variables|Default|GetAggresive%20Material)))

(event Custom|TurnOn
  (Rendering|Components|Light|SetIntensity (Variables|Default|GetSpotLight) (Variables|Default|GetFirstIntensity)))

(event Custom|TurnOff
  (Rendering|Components|Light|SetIntensity (Variables|Default|GetSpotLight) 0.0))

(event EventBeginPlay
  (Variables|Default|SetFirstIntensity (Variables|/Script/Engine.LightComponentBase|GetIntensity (Variables|Default|GetSpotLight))))

(fn ConstructionScript)