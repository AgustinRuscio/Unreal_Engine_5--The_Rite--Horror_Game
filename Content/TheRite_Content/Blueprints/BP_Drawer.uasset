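; BP_Drawer is an interactable drawer that alternately opens and closes on each Interaction event.
; A FlipFlop picks the Open or Close timeline, and CanInteract blocks further input until that timeline finishes.
; Each update lerps the root's relative location from its current value toward that value plus or minus MoveDir, so movement accumulates per tick rather than running between fixed endpoints.
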(event EventInteraction
  (bind _defaultsceneroot (Variables|Default|GetDefaultSceneRoot))
  (bind _defaultsceneroot_2 (Variables|Default|GetDefaultSceneRoot))
  (bind _defaultsceneroot_3 (Variables|Default|GetDefaultSceneRoot))
  (bind _relativelocation (Variables|/Script/Engine.SceneComponent|GetRelativeLocation _defaultsceneroot_3))
  (bind _relativelocation_2 (Variables|/Script/Engine.SceneComponent|GetRelativeLocation _defaultsceneroot_2))
  (if (Variables|Default|GetCanInteract)
    (Utilities|FlowControl|FlipFlop
      (:A
        (Variables|Default|SetCanInteract false)
        (bind _newtrack_0 (Timeline|Open PlayFromStart)
          (:Update
            (Transformation|SetRelativeLocation _defaultsceneroot (Math|Vector|Lerp(Vector) _relativelocation (+ _relativelocation (Variables|Default|GetMoveDir)) _newtrack_0) false false))
          (:Finished
            (Variables|Default|SetCanInteract true :!label _label))))
      (:B
        (Variables|Default|SetCanInteract false)
        (bind _newtrack_0_2 (Timeline|Close PlayFromStart)
          (:Update
            (Transformation|SetRelativeLocation _defaultsceneroot (Math|Vector|Lerp(Vector) _relativelocation_2 (- _relativelocation_2 (Variables|Default|GetMoveDir)) _newtrack_0_2) false false))
          (:Finished
            (goto _label)))))))

(fn ConstructionScript)