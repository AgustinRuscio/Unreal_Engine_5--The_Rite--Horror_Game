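; Trigger volume that plays the TiffanyAlexCue 2D sound when BP_Alex enters its box, then repeats it while Alex stays inside.
; Overlap events toggle an inside flag, and Tick feeds delta time into a SetTimer helper that signals roughly every seven seconds to replay the cue and restart the count.
; Leaving the box clears the flag and timer; despite the asset name, only sound is spawned here.
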(event OnComponentEndOverlap(Box)
  (params (OverlappedComponent :type Primitive%20Component%20Object%20Reference) (OtherActor :type Actor%20Object%20Reference) (OtherComp :type Primitive%20Component%20Object%20Reference) (OtherBodyIndex :type Integer))
  (Utilities|Casting|CastToBP_Alex OtherActor)
  (Variables|Default|SetAlexInside false)
  (Variables|Default|SetTimer 0.0))

(event OnComponentBeginOverlap(Box)
  (params (OverlappedComponent :type Primitive%20Component%20Object%20Reference) (OtherActor :type Actor%20Object%20Reference) (OtherComp :type Primitive%20Component%20Object%20Reference) (OtherBodyIndex :type Integer) (bFromSweep :type Boolean) (SweepResult :type Hit%20Result%20Structure%20%28by%20ref%29))
  (Utilities|Casting|CastToBP_Alex OtherActor)
  (Variables|Default|SetAlexInside true)
  (Audio|SpawnSound2D "/Game/TheRite_Content/Sound/SoundFX/Tiffany/TiffanyAlexCue.TiffanyAlexCue" 1.0 1.0 0.0 0))

(event EventTick
  (params (DeltaSeconds :type Float%20%28single-precision%29))
  (if (Variables|Default|GetAlexInside)
    (bind _newparam (CallFunction|SetTimer DeltaSeconds))
    (if _newparam
      (Variables|Default|SetTimer 0.0)
      (Audio|SpawnSound2D "/Game/TheRite_Content/Sound/SoundFX/Tiffany/TiffanyAlexCue.TiffanyAlexCue" 1.0 1.0 0.0 0))))

(fn ConstructionScript)

(fn SetTimer
  (params (deltaTime :type Float%20%28double-precision%29))
  (bind _output_get (Variables|Default|SetTimer (+ deltaTime (Variables|Default|GetTimer))))
  (return (> _output_get 7.0)))