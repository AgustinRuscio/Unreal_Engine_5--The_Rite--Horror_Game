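; Trigger actor that stages a one-time Tiffany scare when BP_Alex enters its box.
; On overlap it spawns a hidden, non-colliding, stationary BP_Tiffany at InvisibleTiffanySpawner and hands it the waypoints.
; It also reveals the SideTiffany mesh, sets the referenced light's intensity low and plays a heavy-breath sound at that light, then destroys itself.
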(event OnComponentBeginOverlap(Box)
  (params (OverlappedComponent :type Primitive%20Component%20Object%20Reference) (OtherActor :type Actor%20Object%20Reference) (OtherComp :type Primitive%20Component%20Object%20Reference) (OtherBodyIndex :type Integer) (bFromSweep :type Boolean) (SweepResult :type Hit%20Result%20Structure%20%28by%20ref%29))
  (bind _light (Variables|Default|GetLight))
  (bind _invisibletiffanyspawner (Variables|Default|GetInvisibleTiffanySpawner))
  (Utilities|Casting|CastToBP_Alex OtherActor)
  (bind _returnvalue (Game|SpawnActorfromClass "/Game/TheRite_Content/Blueprints/Character/OLD/BP_Tiffany.BP_Tiffany_C" (Math|Transform|MakeTransform (Transformation|GetActorLocation _invisibletiffanyspawner) (Transformation|GetActorRotation _invisibletiffanyspawner) "1.000000,1.000000,1.000000") "Undefined" "MultiplyWithRoot" 0 0))
  (Default|SetData _returnvalue false true false)
  (Default|SetWaypoints _returnvalue (Variables|Default|GetWaypoints))
  (Rendering|SetVisibility (Variables|/Script/Engine.Character|GetMesh (Variables|Default|GetSideTiffany)) true false)
  (Rendering|Components|Light|SetIntensity (Variables|/Script/Engine.Light|GetLightComponent _light) 0.2)
  (Audio|PlaySoundatLocation "/Game/TheRite_Content/Sound/SoundFX/Tiffany/HeavyBreath/HeavyBreathCue.HeavyBreathCue" (Transformation|GetActorLocation _light) "0, 0, 0" 3.0 1.0 0.0 0 0 0 0)
  (Actor|DestroyActor))

(fn ConstructionScript)