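; BP_SoundTrigger is a trigger that plays a sound effect at a set position, limited by a cooldown.
; When Interaction fires while CanSound is true, it clears the flag and plays SoundFX at the OverlapPosition location.
; While the flag is off, Tick accumulates delta time in Timer and re-enables it once CoolDown is reached.
; Timer is never reset, so the cooldown stops delaying replays after it first elapses.
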(event EventInteraction
  (if (Variables|Default|GetCanSound)
    (Variables|Default|SetCanSound false)
    (Audio|PlaySoundatLocation (Variables|Default|GetSoundFX) (.location (Variables|Default|GetOverlapPosition)) "0, 0, 0" 1.0 1.0 0.0 0 0 0 0)))

(event EventTick
  (params (DeltaSeconds :type Float%20%28single-precision%29))
  (if (not (Variables|Default|GetCanSound))
    (Variables|Default|SetTimer (+ DeltaSeconds (Variables|Default|GetTimer)))
    (if (>= (Variables|Default|GetTimer) (Variables|Default|GetCoolDown))
      (Variables|Default|SetCanSound true))))

(fn ConstructionScript)