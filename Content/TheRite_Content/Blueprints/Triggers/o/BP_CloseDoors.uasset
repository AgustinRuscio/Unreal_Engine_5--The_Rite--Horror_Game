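; BP_CloseDoors is a one-shot trigger volume that slams a door and changes the lighting when the player character BP_Alex enters its box.
; On overlap it hard-closes the linked door and switches each linked light to an aggressive or normal material, depending on a flag.
; If a destroyable light is assigned, it destroys that light with a breaking sound, then the trigger destroys itself.
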(event OnComponentBeginOverlap(Box)
  (params (OverlappedComponent :type Primitive%20Component%20Object%20Reference) (OtherActor :type Actor%20Object%20Reference) (OtherComp :type Primitive%20Component%20Object%20Reference) (OtherBodyIndex :type Integer) (bFromSweep :type Boolean) (SweepResult :type Hit%20Result%20Structure%20%28by%20ref%29))
  (bind _destroyablelight (Variables|Default|GetDestroyableLight))
  (Utilities|Casting|CastToBP_Alex OtherActor)
  (Default|HardClosing (Variables|Default|GetDoor))
  (for _array_element (Variables|Default|GetLights)
    (if (Variables|Default|GetAggresiveLights)
      (Default|AggresiveMaterial _array_element)
      (else
        (Default|NormalMaterial _array_element))))
  (Utilities|IsValid _destroyablelight
    (:Is%20Valid
      (Actor|DestroyActor _destroyablelight)
      (Audio|PlaySound2D "/Game/TheRite_Content/Sound/SoundFX/SFX_LightBreaking.SFX_LightBreaking" 1.0 1.0 0.0 0 0))
    (:Is%20Not%20Valid
      _))
  (Actor|DestroyActor))

(fn ConstructionScript)