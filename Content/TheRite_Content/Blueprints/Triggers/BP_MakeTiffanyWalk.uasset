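; One-shot scare trigger that makes Tiffany walk to a target when the player enters its box, once KeyObtein has armed it.
; The overlap starts her movement, turns the BP_Alex camera toward her and plays tension sounds.
; Tick sphere-overlaps around her to collect nearby BP_Light actors as she walks.
; Near the target, chained timelines switch those and preset lights off, then back on, and the trigger destroys itself.
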(event OnComponentBeginOverlap(Box)
  (params (OverlappedComponent :type Primitive%20Component%20Object%20Reference) (OtherActor :type Actor%20Object%20Reference) (OtherComp :type Primitive%20Component%20Object%20Reference) (OtherBodyIndex :type Integer) (bFromSweep :type Boolean) (SweepResult :type Hit%20Result%20Structure%20%28by%20ref%29))
  (if (Variables|Default|GetKeyReady)
    (Utilities|FlowControl|DoOnce false
      (:Completed
        (bind _asbp_alex (Utilities|Casting|CastToBP_Alex OtherActor))
        (Utilities|FlowControl|Sequence
          (:then_0
            ;[1 1 1] Set tifanny Target
            (Default|StartMovement (Variables|Default|GetTiff) (Variables|Default|GetTarget))
            (Variables|Default|Setready true))
          (:then_1
            ;[1 1 1] Make Player Look the enemy
            (Utilities|FlowControl|DoOnce false
              (:Completed
                (Default|CameraTargetting _asbp_alex (Transformation|GetActorLocation (Variables|Default|GetTiff))))))
          (:then_2
            ;[1 1 1] Play all sounds
            (Audio|SpawnSound2D (Variables|Default|GetSound) 1.0 1.0 0.0 0)
            (Audio|SpawnSound2D "/Game/TheRite_Content/Sound/SoundFX/SFX_HeartBeat.SFX_HeartBeat" 1.0 1.0 0.0 0)
            (Audio|SpawnSound2D "/Game/TheRite_Content/Sound/SoundFX/SFX_TiffanyNear.SFX_TiffanyNear" 1.0 1.0 0.0 0)))))))

(event Custom|KeyObtein
  (params (NewTiffany :type BP%20Tiffany%20Object%20Reference))
  (Variables|Default|SetTiff NewTiffany)
  (Variables|Default|SetKeyReady true))

(event EventTick
  (params (DeltaSeconds :type Float%20%28single-precision%29))
  (if (Variables|Default|Getready)
    (bind _tiff (Variables|Default|GetTiff)
      (:then
        (if (> (Math|Vector|Distance(Vector) (Transformation|GetActorLocation (Variables|Default|GetTarget)) (Transformation|GetActorLocation _tiff)) 2e+02)
          ;[1 1 1] Obtein lights
          (bind _tiff_2 (Variables|Default|GetTiff)
            (:then
              (bind (_outactors _returnvalue) (Collision|SphereOverlapActors (Transformation|GetActorLocation _tiff_2) 3e+02 (Utilities|Array|MakeArray "ObjectTypeQuery2") "/Game/TheRite_Content/Blueprints/Others/BP_Light.BP_Light_C"))
              (if _returnvalue
                (for _array_element _outactors
                  (Utilities|Array|Add (Variables|Default|GetLight) (.AsBP%20Light (Utilities|Casting|CastToBP_Light _array_element))))))
            (:else))
          (else
            ;[1 1 1] Turn lights off
            (Timeline|Timeline Play
              (:Update
                (Utilities|FlowControl|Sequence
                  (:then_0
                    (for _array_element_2 (Variables|Default|GetOtherLights)
                      (Default|TurnOff _array_element_2)))
                  (:then_1
                    (for _array_element_3 (Variables|Default|GetLight)
                      (Default|TurnOff _array_element_3)))))
              (:Finished
                (Timeline|Timeline_0 PlayFromStart
                  (:Update
                    (for _array_element_4 (Variables|Default|GetLight)
                      (Default|Turnon _array_element_4))
                    (for _array_element_5 (Variables|Default|GetOtherLights)
                      (Default|Turnon _array_element_5))
                    (Actor|DestroyActor))))))))
      (:else))))

(fn ConstructionScript)