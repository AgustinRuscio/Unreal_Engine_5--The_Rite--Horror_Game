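; Blueprint utility library that gives typed access to The Rite's core framework objects.
; Getters cast the game instance, game state, player controllers (gameplay and menu) and player state to project classes, using index 0 for player lookups.
; Get GS_Menu and Get BP_GS_TheRite both return GS_TheRite.
; Save Settings saves GameUserSettings, then calls SaveGame on the game state for the GameSettings slot.
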(fn GetBPGameInstance
  (bind _asbp_game_instance (Utilities|Casting|CastToBP_GameInstance (Game|GetGameInstance (LocalVariables|Get__WorldContext))))
  (return _asbp_game_instance))

(fn GetGSMenu
  (bind _asgs_the_rite (Utilities|Casting|CastToGS_TheRite (Game|GetGameState (LocalVariables|Get__WorldContext))))
  (return _asgs_the_rite))

(fn SaveSettings
  (bind _gs_menu (CallFunction|GetGSMenu (LocalVariables|Get__WorldContext)))
  (bind _returnvalue (Settings|GetGameUserSettings))
  (Class|GameUserSettings|SaveSettings _returnvalue)
  (Default|SaveGame _gs_menu "GameSettings"))

(fn GetPlayerController
  (bind _asbp_alex_player_controller (Utilities|Casting|CastToBP_AlexPlayerController (Game|GetPlayerController (LocalVariables|Get__WorldContext))))
  (return _asbp_alex_player_controller))

(fn GetPlayerState
  (bind _asbp_player_state_the_rite (Utilities|Casting|CastToBP_PlayerStateTheRite (Game|GetPlayerState (LocalVariables|Get__WorldContext))))
  (return _asbp_player_state_the_rite))

(fn GetBPPCMenu
  (bind _asbp_pc_menu (Utilities|Casting|CastToBP_PC_Menu (Game|GetPlayerController (LocalVariables|Get__WorldContext))))
  (return _asbp_pc_menu))

(fn GetBPGStheRite
  (bind _asgs_the_rite (Utilities|Casting|CastToGS_TheRite (Game|GetGameState (LocalVariables|Get__WorldContext))))
  (return _asgs_the_rite))