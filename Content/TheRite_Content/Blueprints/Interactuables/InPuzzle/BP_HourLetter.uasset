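; Interactable letter puzzle object that plays Alex's last audio and then signals an action, presumably to open a door.
; The Alex on/off events show and hide its BaseWidget.
; Interaction works once: it clears CanInteract, spawns the audio at the actor's location and binds OpenDoor to playback finishing.
; OpenDoor fires the OnActopn dispatcher for any listeners and destroys the letter.
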(event Custom|OpenDoor
  (Default|CallOnActopn)
  (Actor|DestroyActor))

(event EventInteraction
  (if (Variables|Default|GetCan%20Interact)
    (Variables|Default|SetCan%20Interact false)
    (bind _returnvalue (Audio|SpawnSoundatLocation "/Game/TheRite_Content/Sound/Voice/Alex/A_Alex_LastAudio.A_Alex_LastAudio" (Transformation|GetActorLocation) "0, 0, 0" 1.0 1.0 0.0 0 0))
    (EventDispatchers|BindEventtoOnAudioFinished _returnvalue (delegate Custom|OpenDoor))))

(event EventOnAlexon
  (Rendering|SetVisibility (Variables|Default|GetBaseWidget) true false))

(event EventOnAlexOff
  (Rendering|SetVisibility (Variables|Default|GetBaseWidget) false false))

(fn ConstructionScript)