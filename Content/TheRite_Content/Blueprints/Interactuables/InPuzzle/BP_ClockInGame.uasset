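; BP_ClockInGame is an interactable puzzle clock that loads a level once both its Hour and Minutes flags are set.
; On success, a timeline drives an optional nearby spotlight's intensity before a short delay and the level change.
; On failure, Alex plays a first-time wrong-time line or a repeat line, and interaction stays locked until the audio finishes.
; Alex on/off events toggle the base widget's visibility.
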(event Custom|InteractionOnAgain
  (Variables|Default|SetCanInteract true))

(event EventInteraction
  (bind _returnvalue (Transformation|GetActorLocation))
  (bind _nearlight (Variables|Default|GetNearLight))
  (bind _spotlight (Variables|/Game/TheRite_Content/Blueprints/Others/BP_Light.BP_Light_C|GetSpotLight _nearlight))
  (if (Variables|Default|GetCanInteract)
    (Variables|Default|SetCanInteract false)
    (bind (_readr _hour _minutes_) (CallFunction|CheckThings))
    (if _readr
      (Utilities|IsValid _nearlight
        (:Is%20Valid
          (bind _intensitymultiplayer (Timeline|Light PlayFromStart)
            (:Update
              (Rendering|Components|Light|SetIntensity _spotlight (* (Variables|/Script/Engine.LightComponentBase|GetIntensity _spotlight) _intensitymultiplayer)))
            (:Finished
              (Utilities|FlowControl|Delay 1.0 :!label _label)
              (Game|OpenLevel(byObjectReference) (Variables|Default|GetLevel))
              (Actor|DestroyActor))))
        (:Is%20Not%20Valid
          (goto _label)))
      (else
        (if (and (not _hour) (not _minutes_))
          _
          (elif _hour
            _
            (else
              _)))
        (if (== (Variables|Default|GetAudioFirstTime) 0)
          (Variables|Default|SetAudioFirstTime 1)
          (bind _returnvalue_2 (Audio|SpawnSoundatLocation "/Game/TheRite_Content/Sound/Voice/Alex/A_Alex_TimeWorngAudio.A_Alex_TimeWorngAudio" _returnvalue "0, 0, 0" 1.0 1.0 0.0 0 0))
          (EventDispatchers|BindEventtoOnAudioFinished _returnvalue_2 (delegate Custom|InteractionOnAgain))
          (else
            (bind _returnvalue_3 (Audio|SpawnSoundatLocation "/Game/TheRite_Content/Sound/Voice/Alex/A_Alex_IStillDontRemember.A_Alex_IStillDontRemember" _returnvalue "0, 0, 0" 1.0 1.0 0.0 0 0))
            (EventDispatchers|BindEventtoOnAudioFinished _returnvalue_3 (delegate Custom|InteractionOnAgain))))))))

(event EventOnAlexon
  (Rendering|SetVisibility (Variables|Default|GetBaseWidget) true false))

(event EventOnAlexOff
  (Rendering|SetVisibility (Variables|Default|GetBaseWidget) false false))

(fn ConstructionScript)

(fn CheckThings
  (bind _hour (Variables|Default|GetHour))
  (bind _minutes (Variables|Default|GetMinutes))
  (return (and _hour _minutes) _hour _minutes))