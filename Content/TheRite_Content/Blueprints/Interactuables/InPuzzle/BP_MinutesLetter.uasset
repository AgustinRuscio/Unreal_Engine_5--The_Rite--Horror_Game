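; BP_MinutesLetter is an in-puzzle interactable letter that triggers record player audio when picked up.
; Its base widget is shown and hidden by the Alex on/off events.
; Interacting fires the action call, tells the RecordPlayer to play its audio, then destroys the letter.
; An unconnected, one-shot branch that would play the A_TheMinutes sound at the letter's location is left unused.
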(event Custom|a)

(event EventInteraction
  (Default|CallOnAction)
  (Default|PlayAudio (Variables|Default|GetRecord%20Player))
  (Actor|DestroyActor))

(event EventOnAlexOff
  (Rendering|SetVisibility (Variables|Default|GetBaseWidget) false false))

(event EventOnAlexon
  (Rendering|SetVisibility (Variables|Default|GetBaseWidget) true false))

(fn ConstructionScript)