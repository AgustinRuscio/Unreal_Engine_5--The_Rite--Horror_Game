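; BP_Door is a configurable interactable door whose construction script dresses it from variant flags, unless IsException is set.
; It selects double, hospital or standard door meshes and materials, toggles latches and bases, and positions up to two number meshes.
; Key or security card options swap the key mesh and unlock sound, while a separate flag turns bases into card readers.
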(fn ConstructionScript
  (if (not (Variables|Customization|GetIsException))
    (Utilities|FlowControl|Sequence
      (:then_0
        (|SetDoorMesh))
      (:then_1
        (|Showlatch))
      (:then_2
        (|UseKeyOrCard))
      (:then_3
        (|Showbase))
      (:then_4
        (|BaseSecuritycard))
      (:then_5
        (|ShowNumber)))))