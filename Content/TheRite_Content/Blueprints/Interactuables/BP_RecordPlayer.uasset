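; BP_RecordPlayer is an interactable record player that toggles a song on and off.
; On BeginPlay it spawns the song at its location as a paused audio component.
; Interaction alternates play and pause through a FlipFlop, while PlayAudio and StopAudio events set either state directly without updating that FlipFlop.
; Tick rotates the handle (Manija) and record (Disco) by a fixed step per frame while playing.
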(event Custom|Play%20Audio
  (bind _output_get (Variables|Default|SetisPause false))
  (Class|AudioComponent|SetPaused (Variables|Default|GetAudioComponent) _output_get))

(event Custom|Stop%20Audio
  (bind _output_get (Variables|Default|SetisPause true))
  (Class|AudioComponent|SetPaused (Variables|Default|GetAudioComponent) _output_get))

(event EventInteraction
  (bind _audiocomponent (Variables|Default|GetAudioComponent))
  (Utilities|FlowControl|FlipFlop
    (:A
      (bind _output_get (Variables|Default|SetisPause false))
      (Class|AudioComponent|SetPaused _audiocomponent _output_get))
    (:B
      (bind _output_get_2 (Variables|Default|SetisPause true))
      (Class|AudioComponent|SetPaused _audiocomponent _output_get_2))))

(event EventBeginPlay
  (bind _returnvalue (Audio|SpawnSoundatLocation (Variables|Default|GetSong) (Transformation|GetActorLocation) "0, 0, 0" 1.0 1.0 0.0 "/Game/TheRite_Content/Sound/RecordPlayerAttenuation.RecordPlayerAttenuation" 0))
  (bind _output_get (Variables|Default|SetAudioComponent _returnvalue))
  (bind _output_get_2 (Variables|Default|SetisPause true))
  (Class|AudioComponent|SetPaused _output_get _output_get_2))

(event EventTick
  (params (DeltaSeconds :type Float%20%28single-precision%29))
  (if (not (Variables|Default|GetisPause))
    (Transformation|AddLocalRotation (Variables|Default|Getmanija) "0.000000,0.000000,1.000000" false false)
    (Transformation|AddLocalRotation (Variables|Default|Getdisco) "0.000000,1.000000,0.000000" false false)))

(fn ConstructionScript)