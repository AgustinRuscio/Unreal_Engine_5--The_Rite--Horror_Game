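; BP_Key is an interactable key pickup that grants its key to a linked door, with door and zone name assigned through SetDoor and SetZone.
; BeginPlay creates a hidden UI_Key widget labeled with the zone name, while OnAlexon and OnAlexOff toggle BaseWidget's visibility.
; Interaction notifies the door, plays a grab sound, hides the sphere, briefly shows the widget, then destroys the actor.
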(event EventOnAlexon
  (Rendering|SetVisibility (Variables|Default|GetBaseWidget) true false))

(event EventOnAlexOff
  (Rendering|SetVisibility (Variables|Default|GetBaseWidget) false false))

(event EventBeginPlay
  (Utilities|FlowControl|Delay 0.1)
  (bind _returnvalue (UserInterface|CreateWidget "/Game/TheRite_Content/Ui/UI_Key.UI_Key_C"))
  (bind _output_get (Variables|Default|SetUI_Key _returnvalue))
  (Default|SetText _output_get (Variables|Default|GetDoor%20Zone%20Name))
  (Widget|SetVisibility (Variables|Default|GetUI_Key) "Hidden")
  (UserInterface|Viewport|AddtoViewport (Variables|Default|GetUI_Key) 0)
  (Widget|SetVisibility (Variables|Default|GetUI_Key) "Hidden")
  (Development|PrintString "Hello"))

(event EventInteraction
  (bind _ui_key (Variables|Default|GetUI_Key))
  (bind _sphere_0 (Variables|Default|GetSphere_0))
  (Default|ObteinKey (Variables|Default|GetMyDoor))
  (Audio|PlaySoundatLocation "/Game/TheRite_Content/Sound/SoundFX/SFX_GrabItem.SFX_GrabItem" (Transformation|GetActorLocation) "0, 0, 0" 1.0 1.0 0.0 0 0 0 0)
  (Rendering|SetVisibility _sphere_0 false false)
  (Collision|SetCollisionEnabled _sphere_0 "NoCollision")
  (Widget|SetVisibility _ui_key "Visible")
  (Utilities|FlowControl|Delay 2.0)
  (Widget|SetVisibility _ui_key "Hidden")
  (Actor|DestroyActor))

(fn ConstructionScript)

(fn SetDoor
  (params (NewDoor :type BP%20Door%20Object%20Reference))
  (Variables|Default|SetMyDoor NewDoor))

(fn SetZone
  (params (Text :type String))
  (Variables|Default|SetDoor%20Zone%20Name Text))