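; BP_Portrait is an interactable portrait that drops when used and makes a linked key available, once its puzzle is flagged ready.
; While PuzzleReady is set, the OnAlexon and OnAlexOff events show and hide its widget.
; Interaction enables physics on the mesh, shrinks its own sphere to zero, then sets the key ready, enlarges the key's sphere and sets its light intensity.
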(event EventInteraction
  (bind _key (Variables|Default|GetKey))
  (if (Variables|Default|GetPuzzleReady)
    (Physics|SetSimulatePhysics (Variables|Default|GetStaticMesh) true)
    (Components|Sphere|SetSphereRadius (Variables|Default|GetSphere) 0.0 false)
    (Variables|/Game/TheRite_Content/Blueprints/Interactuables/BP_Key.BP_Key_C|SetKeyReady _key true)
    (Components|Sphere|SetSphereRadius (Variables|/Game/TheRite_Content/Blueprints/Abstracts/A_BP_Interactor.A_BP_Interactor_C|GetSphere _key) 165.0 true)
    (Rendering|Components|Light|SetIntensity (Variables|/Game/TheRite_Content/Blueprints/Interactuables/BP_Key.BP_Key_C|GetPointLight _key) 0.05)))

(event EventOnAlexon
  (if (Variables|Default|GetPuzzleReady)
    (Rendering|SetVisibility (Variables|Default|GetBaseWidget) true false)))

(event EventOnAlexOff
  (if (Variables|Default|GetPuzzleReady)
    (Rendering|SetVisibility (Variables|Default|GetBaseWidget) false false)))

(fn ConstructionScript)