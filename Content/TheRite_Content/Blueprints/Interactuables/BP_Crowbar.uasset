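; BP_Crowbar is an interactable crowbar that unlocks a linked Wood object when the player interacts with it.
; On BeginPlay it creates a UI_CrowBar widget, adds it to the viewport and keeps it hidden.
; Interaction calls Unlock on Wood, hides the Cone component and shows the widget briefly.
; After the delay it hides the widget and destroys itself.
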(event EventInteraction
  (Default|Unlock (Variables|Default|GetWood))
  (Rendering|SetVisibility (Variables|Default|GetCone) false false)
  (Widget|SetVisibility (stale EventBeginPlay _output_get) "Visible")
  (Utilities|FlowControl|Delay 2.0)
  (Widget|SetVisibility (stale EventBeginPlay _output_get) "Hidden")
  (Actor|DestroyActor))

(event EventBeginPlay
  (bind _returnvalue (UserInterface|CreateWidget "/Game/TheRite_Content/Ui/UI_CrowBar.UI_CrowBar_C"))
  (bind _output_get (Variables|Default|SetNewVar _returnvalue))
  (UserInterface|Viewport|AddtoViewport _output_get 0)
  (Widget|SetVisibility _output_get "Hidden"))

(fn ConstructionScript)