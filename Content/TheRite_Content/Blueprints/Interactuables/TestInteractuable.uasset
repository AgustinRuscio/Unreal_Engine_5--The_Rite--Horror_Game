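; TestInteractuable is a test interactable actor that reacts when the player collects all items.
; On BeginPlay it casts the player pawn to BP_Alex and binds to its OnAllItemsCollected dispatcher.
; When that fires, it swaps the Cube's material to a cut-stone brick.
; Its Interaction function only prints a debug greeting.
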(event Custom|OnAllItemsCollected_Event
  (Rendering|Material|SetMaterial (Variables|Components|GetCube) 0 "/Game/StarterContent/Materials/M_Brick_Cut_Stone.M_Brick_Cut_Stone"))

(event EventBeginPlay
  (|CallParentFunction)
  (bind _asbp_alex (Utilities|Casting|CastToBP_Alex (Game|Player|GetPlayerPawn 0)))
  (bind _output_get (Variables|Default|SetNewVar_0 _asbp_alex))
  (EventDispatchers|AssignOnAllItemsCollected _output_get (delegate Custom|OnAllItemsCollected_Event)))

(fn ConstructionScript)

(fn Interaction
  (Development|PrintString "Hello")
  (return))