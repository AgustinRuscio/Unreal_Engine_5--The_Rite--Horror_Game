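; Interactable door that a FlipFlop toggles open and closed, with locked and key-required states and timelines rotating door and handles.
; The first keyed use plays an unlock sound whose finish event swings it open.
; Locked attempts jiggle it, flash a UI_Locked widget and play a voice line, muted for about a minute after repeats.
; Separate timelines serve BP_Tiffany overlaps and Open/Close events; LockDoor/UnlockDoor only swap component visibility.
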(event OnComponentBeginOverlap(Sphere1)
  (params (OverlappedComponent :type Primitive%20Component%20Object%20Reference) (OtherActor :type Actor%20Object%20Reference) (OtherComp :type Primitive%20Component%20Object%20Reference) (OtherBodyIndex :type Integer) (bFromSweep :type Boolean) (SweepResult :type Hit%20Result%20Structure%20%28by%20ref%29))
  ;[1 1 1] Tiffany Open Door
  (Utilities|Casting|CastToBP_Tiffany OtherActor)
  (bind _doorfloat (Timeline|Timeline Play)
    (:Update
      (Transformation|SetRelativeRotation (Variables|Default|GetDoor%20itSelf) (Math|Rotator|MakeRotator 0.0 0.0 (Math|Float|Lerp 0.0 9e+01 _doorfloat)) false false))))

(event OnComponentEndOverlap(Sphere1)
  (params (OverlappedComponent :type Primitive%20Component%20Object%20Reference) (OtherActor :type Actor%20Object%20Reference) (OtherComp :type Primitive%20Component%20Object%20Reference) (OtherBodyIndex :type Integer))
  ;[1 1 1] Tiffany Open Door
  (Utilities|Casting|CastToBP_Tiffany OtherActor)
  (bind _doorfloat (Timeline|Timeline Reverse)
    (:Update
      (Transformation|SetRelativeRotation (Variables|Default|GetDoor%20itSelf) (Math|Rotator|MakeRotator 0.0 0.0 (Math|Float|Lerp 0.0 9e+01 _doorfloat)) false false))))

(event Custom|Close
  ;[1 1 1] Open/CloseDoor  Event
  (bind _doorfloat (Timeline|Timeline_1 Reverse)
    (:Update
      (Transformation|SetRelativeRotation (Variables|Default|GetDoor%20itSelf) (Math|Rotator|MakeRotator 0.0 0.0 (Math|Float|Lerp 0.0 9e+01 _doorfloat)) false false))))

(event Custom|CustomEvent
  (Audio|PlaySoundatLocation "/Game/TheRite_Content/Sound/SoundFX/SFX_DoorOpening.SFX_DoorOpening" (Transformation|GetActorLocation) "0, 0, 0" 1.0 1.0 0.0 0 0 0 0)
  (bind _doorfloat (Timeline|Timeline_0 Play)
    (:Update
      (Transformation|SetRelativeRotation (Variables|Default|GetDoor%20itSelf) (Math|Rotator|MakeRotator 0.0 0.0 (Math|Float|Lerp 0.0 9e+01 _doorfloat)) false false))))

(event Custom|Open
  ;[1 1 1] Open/CloseDoor  Event
  (bind _doorfloat (Timeline|Timeline_1 Play)
    (:Update
      (Transformation|SetRelativeRotation (Variables|Default|GetDoor%20itSelf) (Math|Rotator|MakeRotator 0.0 0.0 (Math|Float|Lerp 0.0 9e+01 _doorfloat)) false false))))

(event Custom|Its%20Locked
  ;[1 1 1] Locked Interaction
  (if (Variables|LockedState|GetCanSounditLock)
    (bind _returnvalue (Audio|SpawnSound2D "/Game/TheRite_Content/Sound/Voice/Alex/A_Alex_ItisLocked.A_Alex_ItisLocked" 1.0 1.0 0.0 0))
    (EventDispatchers|BindEventtoOnAudioFinished _returnvalue (delegate Custom|CustomEvent_0)))
  (Utilities|FlowControl|Sequence
    (:then_0
      (Widget|SetVisibility (Variables|LockedState|GetUI_ItsLocked) "Visible")
      (CallFunction|LatchAnim)
      (Utilities|FlowControl|Delay 0.5)
      (Widget|SetVisibility (Variables|LockedState|GetUI_ItsLocked) "Hidden")
      (Variables|LockedState|SetAudioCounterItsLocked (+ (Variables|LockedState|GetAudioCounterItsLocked) 1))
      (if (not (Variables|LockedState|GetCanSounditLock))
        (Variables|Default|SetCanInteract_0 true)))
    (:then_1
      (bind _a (Timeline|Timeline_3 PlayFromStart)
        (:Update
          (Transformation|SetRelativeRotation (Variables|Default|GetDoor%20itSelf) (Math|Rotator|MakeRotator 0.0 0.0 (Math|Float|Lerp 0.0 5.0 _a)) false false))
        (:Finished
          (Audio|PlaySoundatLocation "/Game/TheRite_Content/Sound/SoundFX/SFX_DoorLocked.SFX_DoorLocked" (Transformation|GetActorLocation) "0, 0, 0" 1.0 1.0 0.0 0 0 0 0))))))

(event Custom|CustomEvent_0
  ;[1 1 1] Locked Interaction
  (Variables|Default|SetCanInteract_0 true)
  (if (> (Variables|LockedState|GetAudioCounterItsLocked) 1)
    (Variables|LockedState|SetCanSounditLock false)))

(event Custom|Latch%20Anim
  ;[1 1 1] Anim latch
  (bind _a (Timeline|Timeline_4 PlayFromStart)
    (:Update
      (Transformation|SetRelativeRotation (Variables|Default|GetManija) (Math|Rotator|MakeRotator 0.0 (Math|Float|Lerp 5.0 5e+01 _a) 0.0) false false)
      (Transformation|SetRelativeRotation (Variables|Default|GetManija1) (Math|Rotator|MakeRotator -1.8e+02 (Math|Float|Lerp 5.0 5e+01 _a) 0.0) false false))))

(event EventTick
  (params (DeltaSeconds :type Float%20%28single-precision%29))
  ;[1 1 1] Timer Sound ItsLOcked
  (if (not (Variables|LockedState|GetCanSounditLock))
    (bind _output_get (Variables|LockedState|SetItsLockTimer (+ (Variables|LockedState|GetItsLockTimer) DeltaSeconds)))
    (if (> _output_get 6e+01)
      (Variables|LockedState|SetCanSounditLock true)
      (Variables|LockedState|SetItsLockTimer 0.0))))

(event EventInteraction
  (bind _returnvalue (Transformation|GetActorLocation))
  (bind _firsttimekeysound (Variables|Default|GetFirstTimeKeySound))
  (bind _islocked (Variables|Default|GetIsLocked))
  ;[1 1 1] Interaction
  (if (Variables|Default|GetCanInteract_0)
    (Variables|Default|SetCanInteract_0 false)
    (Utilities|FlowControl|FlipFlop
      (:A
        (if _islocked
          (CallFunction|ItsLocked :!label _label)
          (elif (Variables|Default|GetNeedKey)
            (if (Variables|Default|GetKeyUnlocked)
              (if (== _firsttimekeysound 0)
                (Math|Integer|IncrementInt _firsttimekeysound
                  (:%20%20
                    (Audio|Components|Audio|Play (Variables|Default|GetSFX_DoorUnlocked) 0.0)
                    (Variables|Default|SetCanInteract_0 true :!label _label_2)))
                (else
                  (CallFunction|LatchAnim :!label _label_3)
                  (Audio|PlaySoundatLocation "/Game/TheRite_Content/Sound/SoundFX/SFX_DoorLocked.SFX_DoorLocked" _returnvalue "0, 0, 0" 1.0 1.0 0.0 0 0 0 0)
                  (bind _doorfloat (Timeline|door Play)
                    (:Update
                      (Transformation|SetRelativeRotation (Variables|Default|GetDoor%20itSelf) (Math|Rotator|MakeRotator 0.0 0.0 (Math|Float|Lerp 0.0 9e+01 _doorfloat)) false false))
                    (:Finished
                      (goto _label_2)))))
              (else
                (goto _label)))
            (else
              (goto _label_3)))))
      (:B
        (if _islocked
          (goto _label)
          (else
            (CallFunction|LatchAnim)
            (Audio|PlaySoundatLocation "/Game/TheRite_Content/Sound/SoundFX/SFX_DoorOpening.SFX_DoorOpening" _returnvalue "0, 0, 0" 1.0 1.0 0.0 0 0 0 0)
            (Timeline|door Reverse)))))))

(event EventBeginPlay
  (Variables|Default|SetWidgetVisible true)
  (EventDispatchers|BindEventtoOnAudioFinished (Variables|Default|GetSFX_DoorUnlocked) (delegate Custom|CustomEvent))
  (bind _returnvalue (UserInterface|CreateWidget "/Game/TheRite_Content/Ui/UI_Locked.UI_Locked_C"))
  (bind _output_get (Variables|LockedState|SetUI_ItsLocked _returnvalue))
  (UserInterface|Viewport|AddtoViewport _output_get 0)
  (Widget|SetVisibility _output_get "Hidden"))

(fn ConstructionScript)

(fn ObteinKey
  (Variables|Default|SetKeyUnlocked true))

(fn LockDoor
  (Rendering|SetVisibility (Variables|Default|GetOpenDoor) false false)
  (Rendering|SetVisibility (Variables|Default|GetLockedDoor) true false))

(fn UnlockDoor
  (Rendering|SetVisibility (Variables|Default|GetOpenDoor) true false)
  (Rendering|SetVisibility (Variables|Default|GetLockedDoor) false false))