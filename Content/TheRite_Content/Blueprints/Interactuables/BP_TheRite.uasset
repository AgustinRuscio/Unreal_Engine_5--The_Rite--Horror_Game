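; BP_TheRite is an interactable that loads another level once the clock is ready.
; When ready, interaction plays a confirmation sound, runs a timeline that scales the nearby spotlight's intensity if one is valid, then opens the level after a short delay.
; Otherwise it plays an "I don't have the clock" sound.
; A CanSound flag blocks repeat interactions until that sound or the transition sequence finishes.
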(event Custom|OnAudioFinished_Event
  (Variables|Default|SetCanSound true))

(event EventBeginPlay
  (|CallParentFunction) ; This node is disabled and will not be called.\nDrag off pins to build functionality.
)

(event EventInteraction
  (bind _nearlight (Variables|Default|GetNearLight))
  (bind _spotlight (Variables|/Game/TheRite_Content/Blueprints/Others/BP_Light.BP_Light_C|GetSpotLight _nearlight))
  (if (Variables|Default|GetCanSound)
    (Variables|Default|SetCanSound false)
    (if (Variables|Default|GetClockReady)
      (Audio|SpawnSound2D "/Game/TheRite_Content/Sound/Voice/Alex/A_OkeyLetsGo.A_OkeyLetsGo" 1.0 1.0 0.0 0)
      (Utilities|IsValid _nearlight
        (:Is%20Valid
          (bind _intensitymultiplayer (Timeline|Timeline PlayFromStart)
            (:Update
              (Rendering|Components|Light|SetIntensity _spotlight (* (Variables|/Script/Engine.LightComponentBase|GetIntensity _spotlight) _intensitymultiplayer)))
            (:Finished
              (Utilities|FlowControl|Delay 1.0 :!label _label)
              (Variables|Default|SetCanSound true)
              (Game|OpenLevel(byObjectReference) (Variables|Default|GetLevel)))))
        (:Is%20Not%20Valid
          (goto _label)))
      (else
        (bind _returnvalue (Audio|SpawnSound2D "/Game/TheRite_Content/Sound/Voice/Alex/A_IDontHaveTheClock.A_IDontHaveTheClock" 1.0 1.0 0.0 0))
        (EventDispatchers|AssignOnAudioFinished _returnvalue (delegate Custom|OnAudioFinished_Event))))))

(fn ConstructionScript
  (|CallParentFunction))