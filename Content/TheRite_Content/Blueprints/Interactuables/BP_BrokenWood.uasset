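; BP_BrokenWood is an interactable piece of wood that yields a key once it has been unlocked.
; An Unlock event sets the flag that Interaction checks.
; When unlocked, interaction spawns a BP_Key at the wood's transform, links it to the BPDoor reference and destroys the wood.
; Otherwise it briefly shows a UI_Wood widget, which is created hidden at BeginPlay.
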(event Custom|Unlock
  (Variables|Default|SetUnlocked true))

(event EventInteraction
  (bind _returnvalue (Transformation|GetActorTransform))
  (bind _ui (Variables|Default|GetUi))
  (if (Variables|Default|GetUnlocked)
    (bind _returnvalue_2 (Game|SpawnActorfromClass "/Game/TheRite_Content/Blueprints/Interactuables/BP_Key.BP_Key_C" (Math|Transform|MakeTransform (.location _returnvalue) (.rotation _returnvalue) "1.000000,1.000000,1.000000") "Undefined" "MultiplyWithRoot" 0 0))
    (Default|SetDoor _returnvalue_2 (Variables|Default|GetBP_Door))
    (Actor|DestroyActor)
    (else
      (Widget|SetVisibility _ui "Visible")
      (Utilities|FlowControl|Delay 2.0)
      (Widget|SetVisibility _ui "Hidden"))))

(event EventBeginPlay
  (bind _returnvalue (UserInterface|CreateWidget "/Game/TheRite_Content/Ui/UI_Wood.UI_Wood_C"))
  (bind _output_get (Variables|Default|SetUi _returnvalue))
  (UserInterface|Viewport|AddtoViewport _output_get 0)
  (Widget|SetVisibility _output_get "Hidden"))

(fn ConstructionScript)