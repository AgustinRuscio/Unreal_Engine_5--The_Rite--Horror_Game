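; BP_LockedDoor is an interactable door that responds to interaction with locked feedback instead of opening.
; ItsLocked plays a 2D locked sound while timelines jiggle the handle and nudge the door.
; A CanSound gate blocks repeats until the audio finishes, or after a short delay when sound is disabled, and an optional OnInteraction call fires only once.
; Tick re-enables disabled sound after a minute, though nothing in this graph disables it.
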(event Custom|Its%20Locked
  ;[1 1 1] Locked Interaction
  (if (Variables|LockedState|GetCanSounditLock)
    (bind _returnvalue (Audio|SpawnSound2D "/Game/TheRite_Content/Sound/SoundFX/SFX_DoorLocked.SFX_DoorLocked" 1.0 1.0 0.0 0))
    (EventDispatchers|BindEventtoOnAudioFinished _returnvalue (delegate Custom|CustomEvent_0)))
  (Utilities|FlowControl|Sequence
    (:then_0
      (CallFunction|LatchAnim)
      (Utilities|FlowControl|Delay 0.5)
      (if (not (Variables|LockedState|GetCanSounditLock))
        (Variables|Default|SetCanSound true)))
    (:then_1
      (bind _a (Timeline|Timeline_3 PlayFromStart)
        (:Update
          (Transformation|SetRelativeRotation (Variables|Default|GetDoorItself) (Math|Rotator|MakeRotator 0.0 0.0 (Math|Float|Lerp 0.0 5.0 _a)) false false))))))

(event Custom|CustomEvent_0
  ;[1 1 1] Locked Interaction
  (Variables|Default|SetCanSound true))

(event Custom|Latch%20Anim
  ;[1 1 1] Anim latch
  (bind _a (Timeline|Timeline PlayFromStart)
    (:Update
      (Transformation|SetRelativeRotation (Variables|Default|GetManija) (Math|Rotator|MakeRotator 0.0 (Math|Float|Lerp 5.0 5e+01 _a) 0.0) false false))))

(event EventTick
  (params (DeltaSeconds :type Float%20%28single-precision%29))
  ;[1 1 1] Timer Sound ItsLOcked
  (if (not (Variables|LockedState|GetCanSounditLock))
    (bind _output_get (Variables|LockedState|SetItsLockTimer (+ (Variables|LockedState|GetItsLockTimer) DeltaSeconds)))
    (if (> _output_get 6e+01)
      (Variables|LockedState|SetCanSounditLock true)
      (Variables|LockedState|SetItsLockTimer 0.0))))

(event EventInteraction
  (if (Variables|Default|GetCanSound)
    (Variables|Default|SetCanSound false)
    (CallFunction|ItsLocked)
    (if (Variables|Default|GetHasInteraction)
      (if (not (Variables|Default|GetInteractionDone))
        (Variables|Default|SetInteractionDone true)
        (Default|CallOnInteraction)))))

(fn ConstructionScript)