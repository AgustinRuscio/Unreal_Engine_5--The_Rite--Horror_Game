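; BP_Clock is an interactable clock that shows its widget on OnAlexon, hides it on OnAlexOff, and advances the Rite once used.
; Interaction plays a one-time 2D sound, guarded by CanSound.
; When the audio finishes, a bound callback sets ClockReady on the Rite and destroys the actor.
; An older interaction that granted an item, animated a nearby light and opened a level remains disconnected.
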(event Custom|ClockReady
  (Variables|/Game/TheRite_Content/Blueprints/Interactuables/BP_TheRite.BP_TheRite_C|SetClockReady (Variables|Default|GetRite) true)
  (Actor|DestroyActor))

(event EventInteraction
  (if (Variables|Default|GetCanSound)
    (Variables|Default|SetCanSound false)
    (bind _returnvalue (Audio|SpawnSound2D "/Game/TheRite_Content/Sound/Voice/Alex/A_TheClockFinally.A_TheClockFinally" 1.0 1.0 0.0 0))
    (EventDispatchers|BindEventtoOnAudioFinished _returnvalue (delegate Custom|ClockReady))))

(event EventOnAlexon
  (Rendering|SetVisibility (Variables|Default|GetBaseWidget) true false))

(event EventOnAlexOff
  (Rendering|SetVisibility (Variables|Default|GetBaseWidget) false false))

(fn ConstructionScript)