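; Interactable door that the player drags open while holding interact, with lock and key states.
; Tick line-traces from the player camera to confirm aim, then rotates the door by player input within angle limits.
; Interacting while locked triggers a rattle, UI prompt and optional voice line; first use once key-unlocked plays unlock audio, then swings it open.
; Timelines also drive handle animation, scripted open/close/slam, and automatic opening around BP_Tiffany.
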(event OnComponentBeginOverlap(Sphere1)
  (params (OverlappedComponent :type Primitive%20Component%20Object%20Reference) (OtherActor :type Actor%20Object%20Reference) (OtherComp :type Primitive%20Component%20Object%20Reference) (OtherBodyIndex :type Integer) (bFromSweep :type Boolean) (SweepResult :type Hit%20Result%20Structure%20%28by%20ref%29))
  ;[1 1 1] Tiffany Open Door
  (Utilities|Casting|CastToBP_Tiffany OtherActor)
  (bind _doorfloat (Timeline|Timeline Play)
    (:Update
      (Transformation|SetRelativeRotation (Variables|Default|GetDoorItSelft) (Math|Rotator|MakeRotator 0.0 0.0 (Math|Float|Lerp 0.0 9e+01 _doorfloat)) false false))))

(event OnComponentEndOverlap(Sphere1)
  (params (OverlappedComponent :type Primitive%20Component%20Object%20Reference) (OtherActor :type Actor%20Object%20Reference) (OtherComp :type Primitive%20Component%20Object%20Reference) (OtherBodyIndex :type Integer))
  ;[1 1 1] Tiffany Open Door
  (Utilities|Casting|CastToBP_Tiffany OtherActor)
  (bind _doorfloat (Timeline|Timeline Reverse)
    (:Update
      (Transformation|SetRelativeRotation (Variables|Default|GetDoorItSelft) (Math|Rotator|MakeRotator 0.0 0.0 (Math|Float|Lerp 0.0 9e+01 _doorfloat)) false false))))

(event Custom|HardClosing
  (Audio|SpawnSoundatLocation "/Game/TheRite_Content/Sound/SoundFX/SFX_DoorSlam.SFX_DoorSlam" (Transformation|GetActorLocation) "0, 0, 0" 1.0 1.0 0.0 0 0)
  (bind _doorfloat (Timeline|Timeline_5 Play)
    (:Update
      (Transformation|SetRelativeRotation (Variables|Default|GetDoorItSelft) (Math|Rotator|MakeRotator 0.0 0.0 (Math|Float|Lerp 9e+01 0.0 _doorfloat)) false false))))

(event Custom|CustomEvent
  ;[1 1 1] Begin PLay
  (Audio|PlaySoundatLocation "/Game/TheRite_Content/Sound/SoundFX/SFX_DoorOpening.SFX_DoorOpening" (Transformation|GetActorLocation) "0, 0, 0" 1.0 1.0 0.0 0 0 0 0)
  (bind _doorfloat (Timeline|Timeline_0 Play)
    (:Update
      (Transformation|SetRelativeRotation (Variables|Default|GetDoorItSelft) (Math|Rotator|MakeRotator 0.0 0.0 (Math|Float|Lerp 0.0 9e+01 _doorfloat)) false false))))

(event Custom|Open
  ;[1 1 1] Open/CloseDoor  Event
  (bind _doorfloat (Timeline|Timeline_1 Play)
    (:Update
      (Transformation|SetRelativeRotation (Variables|Default|GetDoorItSelft) (Math|Rotator|MakeRotator 0.0 0.0 (Math|Float|Lerp 0.0 9e+01 _doorfloat)) false false))))

(event Custom|Its%20Locked
  ;[1 1 1] Locked Interaction
  (Utilities|IsValid (Variables|Default|GetLockedSound)
    (:Is%20Valid
      (Default|ForceTalk (Variables|Default|GetPlayer) (Variables|Default|GetLockedSound)))
    (:Is%20Not%20Valid
      _))
  (Utilities|FlowControl|Sequence
    (:then_0
      (Widget|SetVisibility (Variables|LockedState|GetUI_ItsLocked) "Visible")
      (CallFunction|LatchAnim)
      (Timeline|itslocked%202 Play
        (:Finished
          (Widget|SetVisibility (Variables|LockedState|GetUI_ItsLocked) "Hidden")
          (Variables|LockedState|SetAudioCounterItsLocked (+ (Variables|LockedState|GetAudioCounterItsLocked) 1)))))
    (:then_1
      (bind _a (Timeline|Itloscked PlayFromStart)
        (:Update
          (Transformation|SetRelativeRotation (Variables|Default|GetDoorItSelft) (Math|Rotator|MakeRotator 0.0 0.0 (Math|Float|Lerp 0.0 5.0 _a)) false false))
        (:Finished
          (Audio|PlaySoundatLocation "/Game/TheRite_Content/Sound/SoundFX/SFX_DoorLocked.SFX_DoorLocked" (Transformation|GetActorLocation) "0, 0, 0" 1.0 1.0 0.0 0 0 0 0))))))

(event Custom|CheckDragoDoor
  (bind _dooritselft (Variables|Default|GetDoorItSelft))
  (bind _sensitivity (Variables|Default|GetSensitivity))
  (bind _dooritselft_2 (Variables|Default|GetDoorItSelft))
  (bind _front_angle (Variables|Default|GetFront%20Angle))
  (bind _front_angle_2 (Variables|Default|GetFront%20Angle))
  (bind _player (Variables|Default|GetPlayer))
  (bind _doorfloat (Variables|/Game/TheRite_Content/Blueprints/Character/OLD/BP_Alex.BP_Alex_C|GetDoorFloat _player))
  (bind _relativerotation (Variables|/Script/Engine.SceneComponent|GetRelativeRotation _dooritselft_2))
  (bind _returnvalue (* _doorfloat _sensitivity))
  ;[1 0.5208 0.5208] Check Drag
  (if (not (Variables|Default|GetIsLocked))
    (if (Variables|Default|GetNeedKey)
      (if (Variables|Default|GetKeyUnlocked)
        (if (Variables|Default|GetHolding) :!label _label
          (if (Variables|Default|GetIsLookingAtDoor?)
            (if (not (== (.yaw _relativerotation) (Math|Float|ClampAngle (.yaw _relativerotation) _front_angle (* _front_angle -1.0))))
              (CallFunction|Latch (Variables|Default|GetHolding))
              (Transformation|AddLocalRotation (Variables|Default|GetDoorItSelft) (Math|Rotator|MakeRotator 0.0 0.0 _returnvalue) false false)
              (Development|PrintString "local")
              (Development|PrintString (Utilities|String|ToString(Float) _doorfloat))
              (Development|PrintString (Utilities|String|ToString(Float) _returnvalue))
              (elif (>= (.yaw _relativerotation) _front_angle_2)
                (Transformation|SetRelativeRotation _dooritselft (Math|Rotator|MakeRotator 0.0 0.0 (- _front_angle_2 1.0)) false false)
                (Development|PrintString "Frint anglr")
                (else
                  (Transformation|SetRelativeRotation _dooritselft (Math|Rotator|MakeRotator 0.0 0.0 (+ (* _front_angle_2 -1.0) 1.0)) false false)
                  (Development|PrintString "back anglr")))))))
      (else
        (goto _label)))))

(event Custom|Close
  ;[1 1 1] Open/CloseDoor  Event
  (bind _doorfloat (Timeline|Timeline_1 Reverse)
    (:Update
      (Transformation|SetRelativeRotation (Variables|Default|GetDoorItSelft) (Math|Rotator|MakeRotator 0.0 0.0 (Math|Float|Lerp 0.0 9e+01 _doorfloat)) false false))))

(event Custom|CheckIfLookingDoor
  (bind _player (Variables|Default|GetPlayer))
  (bind _camera (Variables|/Game/TheRite_Content/Blueprints/Character/OLD/BP_Alex.BP_Alex_C|GetCamera _player))
  (bind _returnvalue (Transformation|GetWorldLocation _camera))
  ;[1 1 1] CHeck if looking Door
  (bind _output_get (Variables|Default|SetHolding (Variables|/Game/TheRite_Content/Blueprints/Character/OLD/BP_Alex.BP_Alex_C|GetHoldingInteractBTN (Variables|Default|GetPlayer))))
  (if _output_get
    (bind (_outhit _returnvalue_2) (Collision|LineTraceForObjects _returnvalue (+ _returnvalue (* (Math|Vector|GetForwardVector _camera) 3e+02)) (Utilities|Array|MakeArray "ObjectTypeQuery2") false 0 "ForDuration" false))
    (if _returnvalue_2
      (Variables|Default|SetIsLookingAtDoor? (== (.HitActor (Collision|BreakHitResult _outhit)) self))
      (else
        (Variables|Default|SetIsLookingAtDoor? false)))))

(event Custom|Latch
  (params (NewParam :type Boolean))
  (if NewParam
    (bind _a (Timeline|Timeline_6 ReverseFromEnd)
      (:Update
        (Transformation|SetRelativeRotation (Variables|Default|GetManija) (Math|Rotator|MakeRotator 0.0 (Math|Float|Lerp 0.0 5e+01 _a) 0.0) false false)
        (Transformation|SetRelativeRotation (Variables|Default|GetManija1) (Math|Rotator|MakeRotator -1.8e+02 (Math|Float|Lerp 0.0 5e+01 _a) 0.0) false false)))
    (else
      (Timeline|Timeline_6 PlayFromStart))))

(event Custom|Latch%20Anim
  ;[1 1 1] Anim latch
  (bind _a (Timeline|Timeline_4 PlayFromStart)
    (:Update
      (Transformation|SetRelativeRotation (Variables|Default|GetManija) (Math|Rotator|MakeRotator 0.0 (Math|Float|Lerp 5.0 5e+01 _a) 0.0) false false)
      (Transformation|SetRelativeRotation (Variables|Default|GetManija1) (Math|Rotator|MakeRotator -1.8e+02 (Math|Float|Lerp 5.0 5e+01 _a) 0.0) false false))))

(event EventTick
  (params (DeltaSeconds :type Float%20%28single-precision%29))
  ;[1 1 1] Timer Sound ItsLOcked
  (Utilities|FlowControl|Sequence
    (:then_0
      (if (not (Variables|LockedState|GetCanSounditLock))
        (bind _output_get (Variables|LockedState|SetItsLockTimer (+ (Variables|LockedState|GetItsLockTimer) DeltaSeconds)))
        (if (> _output_get 6e+01)
          (Variables|LockedState|SetCanSounditLock true)
          (Variables|LockedState|SetItsLockTimer 0.0))))
    (:then_1
      (CallFunction|CheckDragoDoor))
    (:then_2
      (CallFunction|CheckifLookingDoor))))

(event EventInteraction
  (bind _firsttimekeysound (Variables|Default|GetFirstTimeKeySound))
  (bind _islocked (Variables|Default|GetIsLocked))
  ;[1 1 1] Interaction
  (Utilities|FlowControl|FlipFlop
    (:A
      (if _islocked
        (CallFunction|ItsLocked :!label _label)
        (elif (Variables|Default|GetNeedKey)
          (if (Variables|Default|GetKeyUnlocked)
            (if (== _firsttimekeysound 0)
              (Math|Integer|IncrementInt _firsttimekeysound
                (:%20%20
                  (Audio|Components|Audio|Play (Variables|Default|GetSFX_DoorUnlocked) 0.0))))
            (else
              (goto _label))))))
    (:B
      (if _islocked
        (goto _label)))))

(event EventBeginPlay
  ;[1 1 1] Begin PLay
  (Variables|Default|SetWidgetVisible true)
  (EventDispatchers|BindEventtoOnAudioFinished (Variables|Default|GetSFX_DoorUnlocked) (delegate Custom|CustomEvent))
  (bind _returnvalue (UserInterface|CreateWidget "/Game/TheRite_Content/Ui/UI_Locked.UI_Locked_C"))
  (bind _output_get (Variables|LockedState|SetUI_ItsLocked _returnvalue))
  (UserInterface|Viewport|AddtoViewport _output_get 0)
  (Widget|SetVisibility _output_get "Hidden")
  (bind _returnvalue_2 (Actor|GetActorOfClass "/Game/TheRite_Content/Blueprints/Character/OLD/BP_Alex.BP_Alex_C"))
  (Variables|Default|SetPlayer _returnvalue_2))

(fn ConstructionScript)

(fn ObteinKey
  (Variables|Default|SetKeyUnlocked true))

(fn LockDoor
  (Rendering|SetVisibility (Variables|Default|GetOpenDoor) false false)
  (Rendering|SetVisibility (Variables|Default|GetLockedDoor) true false))

(fn UnlockDoor
  (Rendering|SetVisibility (Variables|Default|GetOpenDoor) true false)
  (Rendering|SetVisibility (Variables|Default|GetLockedDoor) false false))