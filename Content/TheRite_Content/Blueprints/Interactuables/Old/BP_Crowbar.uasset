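; Crowbar pickup interactable that unlocks a referenced Wood object when used.
; OnAlexon and OnAlexOff show and hide its BaseWidget, while BeginPlay creates a hidden UI_CrowBar widget in the viewport.
; Interaction unlocks the Wood, hides the Cone, disables Sphere collision, and briefly displays the crowbar UI before destroying the actor.
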(event EventOnAlexon
  (Rendering|SetVisibility (Variables|Default|GetBaseWidget) true false))

(event EventInteraction
  (Default|Unlock (Variables|Default|GetWood))
  (Rendering|SetVisibility (Variables|Default|GetCone) false false)
  (Collision|SetCollisionEnabled (Variables|Default|GetSphere) "NoCollision")
  (Widget|SetVisibility (stale EventBeginPlay _output_get) "Visible")
  (Utilities|FlowControl|Delay 2.0)
  (Widget|SetVisibility (stale EventBeginPlay _output_get) "Hidden")
  (Actor|DestroyActor))

(event EventBeginPlay
  (bind _returnvalue (UserInterface|CreateWidget "/Game/TheRite_Content/Ui/UI_CrowBar.UI_CrowBar_C"))
  (bind _output_get (Variables|Default|SetUI_CrowBar _returnvalue))
  (UserInterface|Viewport|AddtoViewport _output_get 0)
  (Widget|SetVisibility _output_get "Hidden"))

(event EventOnAlexOff
  (Rendering|SetVisibility (Variables|Default|GetBaseWidget) false false))

(fn ConstructionScript)