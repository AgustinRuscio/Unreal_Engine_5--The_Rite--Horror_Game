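; BP_Letter is an interactable letter, filed under old puzzle assets, that fires an action when used and then removes itself.
; OnAlexon and OnAlexOff show and hide its BaseWidget.
; Interaction shares OpenDoor's path, calling CallOnAction and destroying the actor immediately.
; A disconnected branch would play Alex's first audio once and bind OpenDoor to its finish, but it never runs.
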(event Custom|OpenDoor
  (Default|CallOnAction)
  (Actor|DestroyActor))

(event EventInteraction
  (Default|CallOnAction)
  (Actor|DestroyActor))

(event EventOnAlexon
  (Rendering|SetVisibility (Variables|Default|GetBaseWidget) true false))

(event EventOnAlexOff
  (Rendering|SetVisibility (Variables|Default|GetBaseWidget) false false))

(fn ConstructionScript)