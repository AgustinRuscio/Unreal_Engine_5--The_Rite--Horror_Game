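; BP_HourLetter is an interactable letter puzzle prop, filed among old in-puzzle assets.
; It shows or hides its BaseWidget on the Alex on and off events, and on interaction calls its action and destroys itself.
; A disconnected branch would play the A_TheHour sound once and fire OpenDoor when it finishes, but OpenDoor is empty.
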(event Custom|OpenDoor)

(event EventInteraction
  (Default|CallOnActopn)
  (Actor|DestroyActor))

(event EventOnAlexon
  (Rendering|SetVisibility (Variables|Default|GetBaseWidget) true false))

(event EventOnAlexOff
  (Rendering|SetVisibility (Variables|Default|GetBaseWidget) false false))

(fn ConstructionScript)