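; In-game clock puzzle interactable that sends the player to another level once its time is correct.
; Interaction checks the Hour and Minutes flags; success plays a player voice line and a timeline that ramps spotlight intensity each update, then opens the level and destroys the actor.
; Failure plays a wrong-time line the first time and a different line afterwards.
; Alex on/off events show or hide the base widget.
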(event EventBeginPlay
  (bind _returnvalue (Actor|GetActorOfClass "/Game/TheRite_Content/Blueprints/Character/OLD/BP_Alex.BP_Alex_C"))
  (Variables|Default|SetPlayer _returnvalue))

(event EventInteraction
  (bind _player (Variables|Default|GetPlayer))
  (bind _out_actors (Variables|Default|GetOut%20Actors))
  (bind _spotlight (Variables|/Game/TheRite_Content/Blueprints/Others/BP_Light.BP_Light_C|GetSpotLight _out_actors))
  (bind (_readr _hour _minutes_) (CallFunction|CheckThings))
  (if _readr
    (Default|ForceTalk (Variables|Default|GetPlayer) (Variables|Default|GetImGonnaRealseAudio))
    (Timeline|Timeline PlayFromStart
      (:Update
        (Rendering|Components|Light|SetIntensity _spotlight (+ (Variables|/Script/Engine.LightComponentBase|GetIntensity _spotlight) 2e+02)))
      (:Finished
        (Game|OpenLevel(byObjectReference) (Variables|Default|GetLevel))
        (Actor|DestroyActor)))
    (else
      (if (and (not _hour) (not _minutes_))
        _
        (elif _hour
          _
          (else
            _)))
      (if (== (Variables|Default|GetAudioFirstTime) 0)
        (Variables|Default|SetAudioFirstTime 1)
        (Default|ForceTalk _player (Variables|Default|GetTimeWrongAudio))
        (else
          (Default|ForceTalk _player (Variables|Default|GetStillDontRememberAudio)))))))

(event EventOnAlexon
  (Rendering|SetVisibility (Variables|Default|GetBaseWidget) true false))

(event EventOnAlexOff
  (Rendering|SetVisibility (Variables|Default|GetBaseWidget) false false))

(fn ConstructionScript)

(fn CheckThings
  (bind _hour (Variables|Default|GetHour))
  (bind _minutes (Variables|Default|GetMinutes))
  (return (and _hour _minutes) _hour _minutes))