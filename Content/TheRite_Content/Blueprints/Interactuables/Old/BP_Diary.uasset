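; BP_Diary is an interactable diary pickup, stored in an Old folder, that Alex can collect as a main item.
; Alex-on and Alex-off events show and hide its BaseWidget, presumably as a proximity prompt.
; Interaction passes its Name to Alex's ObteinMainItem.
; Nodes that activate the diary UI and destroy the actor are disconnected and never run.
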(event EventOnAlexon
  (Rendering|SetVisibility (Variables|Default|GetBaseWidget) true false))

(event EventInteraction
  (Default|ObteinMainItem (Variables|Default|GetAlex) (Variables|Default|GetName)))

(event EventOnAlexOff
  (Rendering|SetVisibility (Variables|Default|GetBaseWidget) false false))

(fn ConstructionScript)