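; BP_Clock is an interactable clock pickup, stored under Old, that registers clock progress with the Rite when used.
; Alex on/off events toggle its prompt widget, and BeginPlay assigns its interaction sound.
; Interaction sets ClockReady on the Rite, triggers its key-gain call and destroys the actor.
; A disconnected older interaction granted a main item, animated a nearby light's intensity and opened a level.
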(event Custom|ClockReady
  (bind _rite (Variables|Default|GetRite))
  (Variables|/Game/TheRite_Content/Blueprints/Interactuables/Old/BP_TheRite.BP_TheRite_C|SetClockReady _rite true)
  (Default|CallOnKeyGain _rite)
  (Actor|DestroyActor))

(event EventBeginPlay
  (Variables|Default|SetSoundToSound (Variables|Default|GetSound)))

(event EventInteraction
  (CallFunction|ClockReady))

(event EventOnAlexon
  (Rendering|SetVisibility (Variables|Default|GetBaseWidget) true false))

(event EventOnAlexOff
  (Rendering|SetVisibility (Variables|Default|GetBaseWidget) false false))

(fn ConstructionScript)