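; BP_TheRite is an interactable portal that moves the player to another level once its ClockReady flag is set.
; Interaction, when ready, plays the portal sound and a FadeOut level sequence, then opens the target level when the sequence finishes.
; A key-gain event, also fired on BeginPlay, switches between ready and not-ready sounds, which GetSound returns if WillSound is set.
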(event Custom|ChangeLevel
  (Game|OpenLevel(byObjectReference) (Variables|Default|GetLevel)))

(event Custom|ChangeSound
  (if (Variables|Default|GetClockReady)
    (Variables|Default|SetSoundToSound (Variables|Default|GetClockReadySound))
    (else
      (Variables|Default|SetSoundToSound (Variables|Default|GetClockNotReadySound)))))

(event EventBeginPlay
  (EventDispatchers|BindEventtoOnKeyGain (delegate Custom|ChangeSound))
  (Default|CallOnKeyGain))

(event EventInteraction
  (if (Variables|Default|GetClockReady)
    (Audio|PlaySound2D "/Game/TheRite_Content/Sound/SoundFX/SFX_RitePortal.SFX_RitePortal" 1.0 1.0 0.0 0 0)
    (bind _outactor (Sequencer|Player|CreateLevelSequencePlayer "/Game/TheRite_Content/Sequencecs/FadeOut.FadeOut"))
    (Sequencer|Player|Play (Variables|/Script/LevelSequence.LevelSequenceActor|GetSequencePlayer _outactor) :!class /Script/MovieScene.MovieSceneSequencePlayer)
    (EventDispatchers|BindEventtoOnFinished (Variables|/Script/LevelSequence.LevelSequenceActor|GetSequencePlayer _outactor) (delegate Custom|ChangeLevel))))

(fn ConstructionScript
  (|CallParentFunction))

(fn GetSound
  (if (Variables|Default|GetWillSound)
    (return (Variables|Default|GetSoundToSound))
    (else
      (return 0))))