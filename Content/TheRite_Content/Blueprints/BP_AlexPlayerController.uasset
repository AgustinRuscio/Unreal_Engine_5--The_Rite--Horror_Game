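; Player controller Blueprint that detects whether the player is using a gamepad or another input device.
; Each key press sets the gamepad flag on player 0's AlexPlayerController from the pressed key's type.
; Gamepad presses call CallOnAnyKeyPressed, passing true only for the first press while WasFocus is unset, then false.
; Non-gamepad presses clear WasFocus without making that call, re-arming it for the next gamepad press.
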(event Input|KeyboardEvents|AnyKey
  (params (Key :type Key%20Structure :default "None"))
  (bind _returnvalue (Class|KismetInputLibrary|KeyIsGamepadKey Key))
  (:Pressed
    (bind _asalex_player_controller (Utilities|Casting|CastToAlexPlayerController (Game|GetPlayerController 0)))
    (Class|AlexPlayerController|SetIsGamepad _asalex_player_controller _returnvalue)
    (if _returnvalue
      (if (Variables|Default|GetWasFocus)
        (Default|CallOnAnyKeyPressed false)
        (else
          (Variables|Default|SetWasFocus true)
          (Default|CallOnAnyKeyPressed true)))
      (else
        (Variables|Default|SetWasFocus false)))))

(fn ConstructionScript)