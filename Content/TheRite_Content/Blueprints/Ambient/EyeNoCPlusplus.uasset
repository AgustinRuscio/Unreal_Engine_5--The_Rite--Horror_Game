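; Ambient eye actor that turns its static mesh to track BP_Alex.
; On BeginPlay it caches the BP_Alex actor, then each Tick sets the mesh's relative yaw from a look-at rotation with a fixed offset, zeroing pitch and roll.
; The look-at mixes the mesh's relative location with the target's world location, and rotation snaps because the RInterpTo node is unused.
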(event EventTick
  (params (DeltaSeconds :type Float%20%28single-precision%29))
  (bind _staticmeshcomponent (Variables|Debug|GetStaticMeshComponent))
  (Transformation|SetRelativeRotation _staticmeshcomponent (Math|Rotator|MakeRotator 0.0 0.0 (- (.yaw (Math|Rotator|FindLookatRotation (Variables|/Script/Engine.SceneComponent|GetRelativeLocation _staticmeshcomponent) (Transformation|GetActorLocation (Variables|Default|GetTarget)))) 1e+02)) false false))

(event EventBeginPlay
  (bind _returnvalue (Actor|GetActorOfClass "/Game/TheRite_Content/Blueprints/Character/BP_Alex.BP_Alex_C"))
  (Variables|Default|SetTarget _returnvalue))

(fn ConstructionScript)